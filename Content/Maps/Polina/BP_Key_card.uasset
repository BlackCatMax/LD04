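; BP_Key_card is a key card pickup that the player collects by pressing E.
; A Sphere overlap with the ALS_AnimMan character enables the actor's input and shows a TextRender, and leaving the sphere reverses both.
; Pressing E sets the KeyCard flag on the player character and destroys the actor.
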(event OnComponentBeginOverlap(Sphere)
  (params (OverlappedComponent :type Primitive%20Component%20Object%20Reference) (OtherActor :type Actor%20Object%20Reference) (OtherComp :type Primitive%20Component%20Object%20Reference) (OtherBodyIndex :type Integer) (bFromSweep :type Boolean) (SweepResult :type Hit%20Result%20Structure%20%28by%20ref%29))
  (Utilities|Casting|CastToALS_AnimMan_CharacterBP OtherActor)
  (Input|EnableInput (Game|GetPlayerController 0))
  (Rendering|SetVisibility (Variables|Default|GetTextRender) true false))

(event OnComponentEndOverlap(Sphere)
  (params (OverlappedComponent :type Primitive%20Component%20Object%20Reference) (OtherActor :type Actor%20Object%20Reference) (OtherComp :type Primitive%20Component%20Object%20Reference) (OtherBodyIndex :type Integer))
  (Utilities|Casting|CastToALS_AnimMan_CharacterBP OtherActor)
  (Input|DisableInput (Game|GetPlayerController 0))
  (Rendering|SetVisibility (Variables|Default|GetTextRender) false false))

(event Input|KeyboardEvents|E
  (params (Key :type Key%20Structure :default "None"))
  (:Pressed
    (bind _asals_anim_man_character_bp (Utilities|Casting|CastToALS_AnimMan_CharacterBP (Game|GetPlayerCharacter 0)))
    (Variables|/Game/AdvancedLocomotionV4/Blueprints/CharacterLogic/ALS_AnimMan_CharacterBP.ALS_AnimMan_CharacterBP_C|SetKey_card _asals_anim_man_character_bp true)
    (Actor|DestroyActor)))

(fn ConstructionScript)