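; BP_SniperVictim is a scripted map actor that stages a victim being killed by a sniper shot when its trigger box is overlapped.
; Any overlap spawns a small explosion emitter at a hard-coded world location, then delayed steps play a rifle sound and a neck-break victim animation on Victim.
; AnimationFinished is set and the trigger destroyed only after the delays, making the sequence one-shot from then on.
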(event OnComponentBeginOverlap(TriggerBox)
  (params (OverlappedComponent :type Primitive%20Component%20Object%20Reference) (OtherActor :type Actor%20Object%20Reference) (OtherComp :type Primitive%20Component%20Object%20Reference) (OtherBodyIndex :type Integer) (bFromSweep :type Boolean) (SweepResult :type Hit%20Result%20Structure%20%28by%20ref%29))
  (if (not (Variables|Default|GetAnimationFinished))
    (Effects|SpawnEmitteratLocation "/Game/Game/Particles/GrenadeEXP_default.GrenadeEXP_default" "1066.000000,-14186.000000,3351.000000" "0, 0, 0" "0.200000,0.200000,0.200000")
    (Utilities|FlowControl|Delay 0.5)
    (Audio|PlaySound2D "/Game/Game/Sounds/Guns/AA-50-Beowulf_Sound.AA-50-Beowulf_Sound" 1.0 1.0 0.0 0 0)
    (Utilities|FlowControl|Delay 0.3)
    (Components|Animation|PlayAnimation (Variables|Default|GetVictim) "/Game/AdvancedLocomotionV4/CharacterAssets/Zombie_Character/Animations/Death/Stealth/H2H/Z_Paired_H2H_Stealth_NeckBreak_Vic.Z_Paired_H2H_Stealth_NeckBreak_Vic" false)
    (Variables|Default|SetAnimationFinished true)
    (Components|DestroyComponent (Variables|Default|GetTriggerBox))))

(event EventBeginPlay)

(event Collision|EventActorBeginOverlap
  (params (OtherActor :type Actor%20Object%20Reference)))

(event EventTick
  (params (DeltaSeconds :type Float%20%28single-precision%29)))

(fn ConstructionScript)