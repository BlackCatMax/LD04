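; BP_AntennaActivation is an interactable switch that rotates a big antenna and then opens a shipping container's doors.
; Player overlap with the trigger shows a "Turn on" prompt, enables input and opens a gate for the Interaction action until the antenna is activated.
; Pressing it plays a sound and a timeline that turns the antenna and cylinder with camera shake.
; After a short delay, two timelines swing both doors open.
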(event OnComponentBeginOverlap(Trigger)
  (params (OverlappedComponent :type Primitive%20Component%20Object%20Reference) (OtherActor :type Actor%20Object%20Reference) (OtherComp :type Primitive%20Component%20Object%20Reference) (OtherBodyIndex :type Integer) (bFromSweep :type Boolean) (SweepResult :type Hit%20Result%20Structure%20%28by%20ref%29))
  (if (== OtherActor (Game|GetPlayerCharacter 0))
    (if (not (Variables|Default|GetAntennaFinished))
      (bind _returnvalue (UserInterface|CreateWidget "/Game/AdvancedLocomotionV4/Blueprints/UI/Item_Information_UI.Item_Information_UI_C" (Game|GetPlayerController 0)))
      (Variables|/Game/AdvancedLocomotionV4/Blueprints/UI/Item_Information_UI.Item_Information_UI_C|SetItemName _returnvalue "Turn on")
      (UserInterface|Viewport|AddtoViewport _returnvalue 0)
      (Input|EnableInput (Game|GetPlayerController 0))
      (Utilities|FlowControl|Gate true) ; enters at Open
    )))

(event OnComponentEndOverlap(Trigger)
  (params (OverlappedComponent :type Primitive%20Component%20Object%20Reference) (OtherActor :type Actor%20Object%20Reference) (OtherComp :type Primitive%20Component%20Object%20Reference) (OtherBodyIndex :type Integer))
  (if (== (Game|GetPlayerCharacter 0) OtherActor)
    (Widget|RemovefromParent (stale OnComponentBeginOverlap(Trigger) _returnvalue))
    (Input|DisableInput (Game|GetPlayerController 0))
    (Utilities|FlowControl|Gate true) ; enters at Close
  ))

(event Input|ActionEvents|InputActionInteraction
  (params (Key :type Key%20Structure :default "None"))
  (:Pressed
    (Utilities|FlowControl|Gate true
      (:Exit
        (Widget|RemovefromParent (stale OnComponentBeginOverlap(Trigger) _returnvalue))
        (Audio|PlaySound2D "/Game/Game/Sounds/Button/ButtonPush_S011FO_80_Cue.ButtonPush_S011FO_80_Cue" 1.0 1.0 0.0 0 0)
        (bind _newtrack_0 (Timeline|Antenna%20Rotation Play)
          (:Update
            (Utilities|FlowControl|Sequence
              (:then_0
                (Camera|PlayWorldCameraShake "/Game/Maps/AMalginov/BluePrints/BP_CamShake.BP_CamShake_C" (Transformation|GetWorldLocation (Variables|Default|GetTrigger)) 0.0 1e+03))
              (:then_1
                (Transformation|SetRelativeRotation (Variables|Default|GetCylinder) (Math|Rotator|MakeRotator 0.0 0.0 _newtrack_0) false false))
              (:then_2
                (Transformation|SetRelativeRotation (Variables|Default|GetSM_BigAntenna) (Math|Rotator|MakeRotator 0.0 0.0 _newtrack_0) false false)
                (Variables|Default|SetAntennaFinished true))))
          (:Finished
            (Utilities|FlowControl|Delay 2.0)
            (Utilities|FlowControl|Sequence
              (:then_0
                (bind _newtrack_0_2 (Timeline|Left%20Door%20Rotation Play)
                  (:Update
                    (Transformation|SetRelativeRotation (Variables|Default|GetSM_Container_LeftDoor) (Math|Rotator|MakeRotator 0.0 0.0 _newtrack_0_2) false false))))
              (:then_1
                (bind _newtrack_0_3 (Timeline|Right%20Door%20Rotation Play)
                  (:Update
                    (Transformation|SetRelativeRotation (Variables|Default|GetSM_Container_RightDoor) (Math|Rotator|MakeRotator 0.0 0.0 _newtrack_0_3) false false)))))))))))

(fn ConstructionScript)