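; BP_Football is a goal actor for a football mini-game that rewards the first goal scored.
; When its Trigger overlaps the football ball mesh, a Goal flag ensures the reward fires only once.
; Scoring spawns confetti Niagara at a hard-coded world position, plays a 2D sound and spawns a BP_ShopItem_5 at the SpawnLocation component.
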(event OnComponentBeginOverlap(Trigger)
  (params (OverlappedComponent :type Primitive%20Component%20Object%20Reference) (OtherActor :type Actor%20Object%20Reference) (OtherComp :type Primitive%20Component%20Object%20Reference) (OtherBodyIndex :type Integer) (bFromSweep :type Boolean) (SweepResult :type Hit%20Result%20Structure%20%28by%20ref%29))
  (if (== OtherComp (Variables|Default|GetSM_Football_ball))
    (if (not (Variables|Default|GetGoal))
      (Niagara|SpawnSystematLocation "/Game/Maps/AMalginov/BluePrints/NS_confetti_System.NS_confetti_System" "-3006.000000,-9552.000000,2615.000000")
      (Audio|PlaySound2D "/Game/Maps/AMalginov/BluePrints/Sound_Pipe.Sound_Pipe" 1.0 1.0 0.0 0 0)
      (Variables|Default|SetGoal true)
      (Game|SpawnActorfromClass "/Game/Maps/AMalginov/BluePrints/BP_ShopItem_5.BP_ShopItem_5_C" (Math|Transform|MakeTransform (Transformation|GetWorldLocation (Variables|Default|GetSpawnLocation)) "0.000000,-75.000000,0.000000" "1.000000,1.000000,1.000000") "Undefined" 0 0))))

(event EventBeginPlay)

(event EventTick
  (params (DeltaSeconds :type Float%20%28single-precision%29)))

(fn ConstructionScript)