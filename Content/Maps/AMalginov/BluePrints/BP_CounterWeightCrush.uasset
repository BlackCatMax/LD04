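; BP_CounterWeightCrush is a scripted level hazard: a cable-hung counterweight that falls when the player approaches.
; An outer warning zone, Trigger3, shakes the weight with a timeline that restarts at its end position while the player overlaps it.
; Trigger destroys that zone, detaches the cable with effects, and enables physics on the weight for twelve seconds, once only.
; Trigger2 detects the falling weight and plays explosion effects for the landing.
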(event OnComponentBeginOverlap(Trigger)
  (params (OverlappedComponent :type Primitive%20Component%20Object%20Reference) (OtherActor :type Actor%20Object%20Reference) (OtherComp :type Primitive%20Component%20Object%20Reference) (OtherBodyIndex :type Integer) (bFromSweep :type Boolean) (SweepResult :type Hit%20Result%20Structure%20%28by%20ref%29))
  ;[1 1 1] Cable break
  (if (== OtherActor (Game|GetPlayerCharacter 0))
    (Components|DestroyComponent (Variables|Default|GetTrigger3))
    (if (not (Variables|Default|GetTriggerOverlaped))
      (Variables|Default|SetTriggerOverlaped true)
      (bind _output_get (Variables|Default|SetCounterweightLocation (Transformation|GetWorldLocation (Variables|Default|GetSM_Counterweight))))
      (Effects|SpawnEmitteratLocation "/Game/Game/Particles/GrenadeEXP_air.GrenadeEXP_air" (+ _output_get "0.000000,0.000000,50.000000") "0, 0, 0" "0.100000,0.100000,0.100000")
      (Audio|PlaySoundatLocation "/Game/AdvancedLocomotionV4/Audio/Bow/BOW_Hit_Cue.BOW_Hit_Cue" (+ _output_get "0.000000,0.000000,50.000000") "0, 0, 0" 3.0 1.0 0.0 0 0 0 0)
      (Physics|SetSimulatePhysics (Variables|Default|GetSM_Counterweight) true)
      (Variables|/Script/CableComponent.CableComponent|SetbAttachEnd (Variables|Default|GetCable) false)
      (Utilities|FlowControl|Delay 12.0)
      (Physics|SetSimulatePhysics (Variables|Default|GetSM_Counterweight) false))))

(event OnComponentBeginOverlap(Trigger2)
  (params (OverlappedComponent :type Primitive%20Component%20Object%20Reference) (OtherActor :type Actor%20Object%20Reference) (OtherComp :type Primitive%20Component%20Object%20Reference) (OtherBodyIndex :type Integer) (bFromSweep :type Boolean) (SweepResult :type Hit%20Result%20Structure%20%28by%20ref%29))
  ;[1 1 1] Landing
  (if (== OtherComp (Variables|Default|GetSM_Counterweight))
    (bind _output_get (Variables|Default|SetCounterweightLocation (Transformation|GetWorldLocation (Variables|Default|GetSM_Counterweight))))
    (Effects|SpawnEmitteratLocation "/Game/Game/Particles/GrenadeEXP_air.GrenadeEXP_air" (- _output_get "0.000000,0.000000,500.000000") "0, 0, 0" "0.800000,0.800000,0.800000")
    (Audio|PlaySoundatLocation "/Game/Game/Sounds/Grenade/Grenade_Explosion_Cue.Grenade_Explosion_Cue" (- _output_get "0.000000,0.000000,500.000000") "0, 0, 0" 0.5 1.0 0.0 0 0 0 0)))

(event OnComponentBeginOverlap(Trigger3)
  (params (OverlappedComponent :type Primitive%20Component%20Object%20Reference) (OtherActor :type Actor%20Object%20Reference) (OtherComp :type Primitive%20Component%20Object%20Reference) (OtherBodyIndex :type Integer) (bFromSweep :type Boolean) (SweepResult :type Hit%20Result%20Structure%20%28by%20ref%29))
  ;[1 1 1] Shaking
  (if (== OtherActor (Game|GetPlayerCharacter 0))
    (bind _newtrack_1 (Timeline|Shaking Play)
      (:Update
        (bind _output_get (Variables|Default|SetShakePosition _newtrack_1))
        (Transformation|SetRelativeLocation (Variables|Default|GetSM_Counterweight) (Math|Vector|MakeVector 0.0 _output_get 0.0) false false)
        (if (== (Variables|Default|GetShakeEndPosition) (Variables|Default|GetShakePosition))
          (Timeline|Shaking PlayFromStart))))))

(event OnComponentEndOverlap(Trigger3)
  (params (OverlappedComponent :type Primitive%20Component%20Object%20Reference) (OtherActor :type Actor%20Object%20Reference) (OtherComp :type Primitive%20Component%20Object%20Reference) (OtherBodyIndex :type Integer))
  ;[1 1 1] Shaking
  (if (== (Game|GetPlayerCharacter 0) OtherActor)
    (bind _newtrack_1 (Timeline|Shaking Stop)
      (:Update
        (bind _output_get (Variables|Default|SetShakePosition _newtrack_1))
        (Transformation|SetRelativeLocation (Variables|Default|GetSM_Counterweight) (Math|Vector|MakeVector 0.0 _output_get 0.0) false false)
        (if (== (Variables|Default|GetShakeEndPosition) (Variables|Default|GetShakePosition))
          (Timeline|Shaking PlayFromStart))))))

(fn ConstructionScript)