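; BP_Barman is an interactable barman NPC that gives a fetch quest and swaps the requested item for an ID card.
; Entering its trigger shows an Item_Information_UI prompt, enables input and opens a gate for the Interaction press.
; Pressing it plays a mumble sound and shows text-render dialogue chosen by quest state, stored in local booleans and flags on ALS_AnimMan_CharacterBP.
; Leaving removes the prompt and closes the gate.
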(event OnComponentBeginOverlap(Trigger)
  (params (OverlappedComponent :type Primitive%20Component%20Object%20Reference) (OtherActor :type Actor%20Object%20Reference) (OtherComp :type Primitive%20Component%20Object%20Reference) (OtherBodyIndex :type Integer) (bFromSweep :type Boolean) (SweepResult :type Hit%20Result%20Structure%20%28by%20ref%29))
  (bind _returnvalue (Game|GetPlayerCharacter 0))
  (if (== OtherActor _returnvalue)
    (bind _asals_anim_man_character_bp (Utilities|Casting|CastToALS_AnimMan_CharacterBP _returnvalue))
    (bind _returnvalue_2 (UserInterface|CreateWidget "/Game/AdvancedLocomotionV4/Blueprints/UI/Item_Information_UI.Item_Information_UI_C" (Game|GetPlayerController 0)))
    (if (Variables|/Game/AdvancedLocomotionV4/Blueprints/CharacterLogic/ALS_AnimMan_CharacterBP.ALS_AnimMan_CharacterBP_C|GetBarmanItem _asals_anim_man_character_bp)
      (if (Variables|Default|GetBarmanGaveQuest)
        (Variables|/Game/AdvancedLocomotionV4/Blueprints/UI/Item_Information_UI.Item_Information_UI_C|SetItemName _returnvalue_2 "Give the item to Barman")
        (else
          (Variables|/Game/AdvancedLocomotionV4/Blueprints/UI/Item_Information_UI.Item_Information_UI_C|SetItemName _returnvalue_2 "Talk to Barman" :!label _label)))
      (else
        (goto _label)))
    (UserInterface|Viewport|AddtoViewport _returnvalue_2 0)
    (Input|EnableInput (Game|GetPlayerController 0))
    (Utilities|FlowControl|Gate true) ; enters at Open
  ))

(event OnComponentEndOverlap(Trigger)
  (params (OverlappedComponent :type Primitive%20Component%20Object%20Reference) (OtherActor :type Actor%20Object%20Reference) (OtherComp :type Primitive%20Component%20Object%20Reference) (OtherBodyIndex :type Integer))
  (bind _returnvalue (Game|GetPlayerController 0))
  (bind _returnvalue_2 (Game|GetPlayerCharacter 0))
  (if (== _returnvalue_2 OtherActor)
    (Widget|RemovefromParent (stale OnComponentBeginOverlap(Trigger) _returnvalue_2))
    (Rendering|SetVisibility (Variables|Default|GetTextRender1) false true)
    (Input|DisableInput _returnvalue)
    (Utilities|FlowControl|Gate true) ; enters at Close
  ))

(event Input|ActionEvents|InputActionInteraction
  (params (Key :type Key%20Structure))
  (:Pressed
    (Utilities|FlowControl|Gate true :!label _label
      (:Exit
        (Widget|RemovefromParent (stale _returnvalue))
        (Input|DisableInput (Game|GetPlayerController 0))
        (Rendering|SetVisibility (Variables|Default|GetTextRender1) false false)
        (Rendering|SetVisibility (Variables|Default|GetPlane1) true true)
        (Audio|Components|Audio|Stop (Variables|Default|Get2DSound))
        (Audio|PlaySoundatLocation "/Game/Maps/AMalginov/Sounds/Soound_Man-mumble_Cue.Soound_Man-mumble_Cue" (Transformation|GetWorldLocation (Variables|Default|GetSoundLocation)) "0, 0, 0" 1.0 1.0 0.0 0 0 0 0)
        (Variables|Default|Set2DSound 0)
        (Utilities|FlowControl|Delay 0.1)
        (bind _asals_anim_man_character_bp (Utilities|Casting|CastToALS_AnimMan_CharacterBP (Game|GetPlayerCharacter 0)))
        (if (Variables|Default|GetBarmanHasItem)
          (Rendering|SetVisibility (Variables|Default|GetTextRender3) true true :!label _label_2)
          (elif (Variables|/Game/AdvancedLocomotionV4/Blueprints/CharacterLogic/ALS_AnimMan_CharacterBP.ALS_AnimMan_CharacterBP_C|GetBarmanItem _asals_anim_man_character_bp)
            (if (Variables|Default|GetBarmanGaveQuest)
              (Variables|/Game/AdvancedLocomotionV4/Blueprints/CharacterLogic/ALS_AnimMan_CharacterBP.ALS_AnimMan_CharacterBP_C|SetBarmanItem _asals_anim_man_character_bp false)
              (Variables|/Game/AdvancedLocomotionV4/Blueprints/CharacterLogic/ALS_AnimMan_CharacterBP.ALS_AnimMan_CharacterBP_C|SetIDcard _asals_anim_man_character_bp true)
              (Variables|Default|SetBarmanHasItem true)
              (goto _label_2)
              (else
                (Rendering|SetVisibility (Variables|Default|GetTextRender1) true false)
                (Variables|Default|SetBarmanGaveQuest true)
                (bind _asals_anim_man_character_bp_2 (Utilities|Casting|CastToALS_AnimMan_CharacterBP (Game|GetPlayerCharacter 0)))
                (bind _returnvalue (UserInterface|CreateWidget "/Game/AdvancedLocomotionV4/Blueprints/UI/Item_Information_UI.Item_Information_UI_C" (Game|GetPlayerController 0)))
                (if (Variables|/Game/AdvancedLocomotionV4/Blueprints/CharacterLogic/ALS_AnimMan_CharacterBP.ALS_AnimMan_CharacterBP_C|GetBarmanItem _asals_anim_man_character_bp_2)
                  (if (Variables|Default|GetBarmanGaveQuest)
                    (Variables|/Game/AdvancedLocomotionV4/Blueprints/UI/Item_Information_UI.Item_Information_UI_C|SetItemName _returnvalue "Give the item to Barman")
                    (else
                      (Variables|/Game/AdvancedLocomotionV4/Blueprints/UI/Item_Information_UI.Item_Information_UI_C|SetItemName _returnvalue "Talk to Barman" :!label _label_3)))
                  (else
                    (goto _label_3)))
                (UserInterface|Viewport|AddtoViewport _returnvalue 0)
                (Input|EnableInput (Game|GetPlayerController 0))
                (goto _label Open)))
            (else
              (Rendering|SetVisibility (Variables|Default|GetTextRender1) true false)
              (Variables|Default|SetBarmanGaveQuest true))))))))

(fn ConstructionScript)