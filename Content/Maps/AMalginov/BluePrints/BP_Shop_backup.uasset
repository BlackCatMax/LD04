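; BP_Shop_backup is a shopkeeper actor the player can talk to by pressing Interaction inside its trigger.
; Entering as ALS_AnimMan_CharacterBP shows an Item_Information_UI prompt, enables input and opens a gate for the key press.
; Interacting removes the prompt, reveals three planes and two text renders, and plays a mumbling voice cue.
; When the player leaves, everything hides, input is disabled and the gate closes.
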(event OnComponentBeginOverlap(Trigger)
  (params (OverlappedComponent :type Primitive%20Component%20Object%20Reference) (OtherActor :type Actor%20Object%20Reference) (OtherComp :type Primitive%20Component%20Object%20Reference) (OtherBodyIndex :type Integer) (bFromSweep :type Boolean) (SweepResult :type Hit%20Result%20Structure%20%28by%20ref%29))
  (bind _asals_anim_man_character_bp (Utilities|Casting|CastToALS_AnimMan_CharacterBP OtherActor))
  (bind _returnvalue (UserInterface|CreateWidget "/Game/AdvancedLocomotionV4/Blueprints/UI/Item_Information_UI.Item_Information_UI_C" (Game|GetPlayerController 0)))
  (Variables|/Game/AdvancedLocomotionV4/Blueprints/UI/Item_Information_UI.Item_Information_UI_C|SetItemName _returnvalue "Talk to the shopkeeper")
  (UserInterface|Viewport|AddtoViewport _returnvalue 0)
  (Input|EnableInput (Game|GetPlayerController 0))
  (Utilities|FlowControl|Gate true) ; enters at Open
)

(event OnComponentEndOverlap(Trigger)
  (params (OverlappedComponent :type Primitive%20Component%20Object%20Reference) (OtherActor :type Actor%20Object%20Reference) (OtherComp :type Primitive%20Component%20Object%20Reference) (OtherBodyIndex :type Integer))
  (if (== OtherActor (Game|GetPlayerCharacter 0))
    (Widget|RemovefromParent (stale OnComponentBeginOverlap(Trigger) _returnvalue))
    (Rendering|SetVisibility (Variables|Default|GetTextRender1) false false)
    (Input|DisableInput (Game|GetPlayerController 0))
    (Utilities|FlowControl|Gate true) ; enters at Close
  ))

(event Input|ActionEvents|InputActionInteraction
  (params (Key :type Key%20Structure :default "None"))
  (:Pressed
    (Utilities|FlowControl|Gate true
      (:Exit
        (Widget|RemovefromParent (stale OnComponentBeginOverlap(Trigger) _returnvalue))
        (Rendering|SetVisibility (Variables|Default|GetPlane1) true false)
        (Audio|PlaySoundatLocation "/Game/Maps/AMalginov/BluePrints/Sound_Mumbling-male-_short__Cue.Sound_Mumbling-male-_short__Cue" (Transformation|GetWorldLocation (Variables|Default|GetSoundLocation)) "0, 0, 0" 3.0 1.0 0.0 0 0 0 0)
        (Rendering|SetVisibility (Variables|Default|GetTextRender1) true false)))))

(fn ConstructionScript)