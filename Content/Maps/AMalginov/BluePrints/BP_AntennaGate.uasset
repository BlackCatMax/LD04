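; Antenna gate that the player unlocks with an ID card and a four-press numpad password.
; The trigger shows a prompt and, if the character has the card, enables Interaction, which animates a swipe and arms the keypad.
; NumPad 1-4 share one check against Password by PasswordIndex, with timelines pressing buttons that turn green or red.
; Wrong presses or leaving reset the keypad; the final correct press swings the door open with sounds.
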(event OnComponentBeginOverlap(Trigger)
  (params (OverlappedComponent :type Primitive%20Component%20Object%20Reference) (OtherActor :type Actor%20Object%20Reference) (OtherComp :type Primitive%20Component%20Object%20Reference) (OtherBodyIndex :type Integer) (bFromSweep :type Boolean) (SweepResult :type Hit%20Result%20Structure%20%28by%20ref%29))
  (bind _card (Variables|Default|GetCard))
  (bind _card_2 (Variables|Default|GetCard))
  (bind _door (Variables|Default|GetDoor))
  (bind _returnvalue (Transformation|GetWorldLocation _door))
  (if (== OtherActor (Game|GetPlayerCharacter 0))
    (if (not (Variables|Default|GetDoorOpened))
      (bind _asals_anim_man_character_bp (Utilities|Casting|CastToALS_AnimMan_CharacterBP (Game|GetPlayerCharacter 0)))
      (bind _returnvalue_2 (UserInterface|CreateWidget "/Game/AdvancedLocomotionV4/Blueprints/UI/Item_Information_UI.Item_Information_UI_C" (Game|GetPlayerController 0)))
      (if (Variables|/Game/AdvancedLocomotionV4/Blueprints/CharacterLogic/ALS_AnimMan_CharacterBP.ALS_AnimMan_CharacterBP_C|GetIDcard _asals_anim_man_character_bp)
        (Variables|/Game/AdvancedLocomotionV4/Blueprints/UI/Item_Information_UI.Item_Information_UI_C|SetItemName _returnvalue_2 "Use ID Card")
        (UserInterface|Viewport|AddtoViewport _returnvalue_2 0)
        (Input|EnableInput (Game|GetPlayerController 0))
        (Utilities|FlowControl|Gate true) ; enters at Open
        (else
          (Variables|/Game/AdvancedLocomotionV4/Blueprints/UI/Item_Information_UI.Item_Information_UI_C|SetItemName _returnvalue_2 "Need ID card")
          (Variables|/Game/AdvancedLocomotionV4/Blueprints/UI/Item_Information_UI.Item_Information_UI_C|SetIconHidden _returnvalue_2 true)
          (UserInterface|Viewport|AddtoViewport _returnvalue_2 0))))))

(event OnComponentEndOverlap(Trigger)
  (params (OverlappedComponent :type Primitive%20Component%20Object%20Reference) (OtherActor :type Actor%20Object%20Reference) (OtherComp :type Primitive%20Component%20Object%20Reference) (OtherBodyIndex :type Integer))
  (bind _card (Variables|Default|GetCard))
  (bind _card_2 (Variables|Default|GetCard))
  (bind _door (Variables|Default|GetDoor))
  (bind _returnvalue (Transformation|GetWorldLocation _door))
  (if (== (Game|GetPlayerCharacter 0) OtherActor)
    (Variables|Default|SetReadyForPassword false)
    (if (Variables|Default|GetDoorOpened)
      _
      (else
        (Rendering|SetVisibility (Variables|Default|GetTextMain2) false false)
        (Rendering|SetVisibility (Variables|Default|GetTextMain1) true false)))
    (Widget|RemovefromParent (stale OnComponentBeginOverlap(Trigger) _returnvalue_2))
    (Utilities|FlowControl|Sequence
      (:then_0
        (Input|DisableInput (Game|GetPlayerController 0))
        (Utilities|FlowControl|Gate true) ; enters at Close
      )
      (:then_1
        (Rendering|SetVisibility (Variables|Default|GetTextButton1) true false)
        (Rendering|SetVisibility (Variables|Default|GetTextButton1Green) false false)
        (Variables|Default|SetPasswordIndex 0)
        (Utilities|FlowControl|Sequence
          (:then_0
            (if (Utilities|Array|Get(acopy) (Variables|Default|GetGreenButtons))
              (bind _newtrack_0 (Timeline|Pressing%201 ReverseFromEnd)
                (:Update
                  (Transformation|SetRelativeTransform (Variables|Default|GetButton1) (Math|Transform|MakeTransform (Math|Vector|MakeVector 0.0 _newtrack_0 0.0) "0, 0, 0" "1.000000,1.000000,1.000000") false false)))
              (elif (== (Variables|Default|GetNumPressed) 1)
                (Timeline|Pressing%201 ReverseFromEnd)
                (else
                  (Utilities|FlowControl|Delay 0.001 :!label _label)
                  (for (_ _array_index) (Variables|Default|GetGreenButtons)
                    (Utilities|Array|SetArrayElem (Variables|Default|GetGreenButtons) _array_index false))))))
          (:then_1
            (if (Utilities|Array|Get(acopy) (Variables|Default|GetGreenButtons) 1)
              (bind _newtrack_0_2 (Timeline|Pressing%202 ReverseFromEnd)
                (:Update
                  (Transformation|SetRelativeTransform (Variables|Default|GetButton2) (Math|Transform|MakeTransform (Math|Vector|MakeVector 123.529412 _newtrack_0_2 0.0) "0, 0, 0" "1.000000,1.000000,1.000000") false false)))
              (elif (== (Variables|Default|GetNumPressed) 2)
                (Timeline|Pressing%202 ReverseFromEnd)
                (else
                  (goto _label)))))
          (:then_2
            (if (Utilities|Array|Get(acopy) (Variables|Default|GetGreenButtons) 2)
              (bind _newtrack_0_3 (Timeline|Pressing%203 ReverseFromEnd)
                (:Update
                  (Transformation|SetRelativeTransform (Variables|Default|GetButton3) (Math|Transform|MakeTransform (Math|Vector|MakeVector 0.0 _newtrack_0_3 -135.294116) "0, 0, 0" "1.000000,1.000000,1.000000") false false)))
              (elif (== (Variables|Default|GetNumPressed) 3)
                (Timeline|Pressing%203 ReverseFromEnd)
                (else
                  (goto _label)))))
          (:then_3
            (if (Utilities|Array|Get(acopy) (Variables|Default|GetGreenButtons) 3)
              (bind _newtrack_0_4 (Timeline|Pressing%204 ReverseFromEnd)
                (:Update
                  (Transformation|SetRelativeTransform (Variables|Default|GetButton4) (Math|Transform|MakeTransform (Math|Vector|MakeVector 123.52941 _newtrack_0_4 -135.294116) "0, 0, 0" "1.000000,1.000000,1.000000") false false)))
              (elif (== (Variables|Default|GetNumPressed) 4)
                (Timeline|Pressing%204 ReverseFromEnd)
                (else
                  (goto _label))))))))))

(event Input|ActionEvents|InputActionInteraction
  (params (Key :type Key%20Structure :default "None"))
  (bind _card (Variables|Default|GetCard))
  (bind _card_2 (Variables|Default|GetCard))
  (bind _door (Variables|Default|GetDoor))
  (bind _returnvalue (Transformation|GetWorldLocation _door))
  (:Pressed
    (Utilities|FlowControl|Gate true :!label _label
      (:Exit
        (Audio|PlaySound2D "/Game/Maps/AMalginov/BluePrints/Sound_Card-swipe.Sound_Card-swipe" 1.0 1.0 0.0 0 0)
        (Utilities|FlowControl|Sequence
          (:then_0
            (Variables|/Game/AdvancedLocomotionV4/Blueprints/UI/Item_Information_UI.Item_Information_UI_C|SetIconHidden (stale OnComponentBeginOverlap(Trigger) _returnvalue_2) true)
            (Utilities|FlowControl|Delay 1.0)
            (Rendering|SetVisibility (Variables|Default|GetTextMain1) false false)
            (Rendering|SetVisibility (Variables|Default|GetTextMain2) true false)
            (Variables|/Game/AdvancedLocomotionV4/Blueprints/UI/Item_Information_UI.Item_Information_UI_C|SetItemName (stale OnComponentBeginOverlap(Trigger) _returnvalue_2) "Press Numpad")
            (Variables|/Game/AdvancedLocomotionV4/Blueprints/UI/Item_Information_UI.Item_Information_UI_C|SetItemComment (stale OnComponentBeginOverlap(Trigger) _returnvalue_2) "[7] [8] [9] 
[4] [5] [6] 
[1] [2] [3]")
            (Variables|Default|SetReadyForPassword true)
            (Utilities|FlowControl|Gate true) ; enters at Open
          )
          (:then_1
            (Rendering|SetVisibility (Variables|Default|GetCard) true false)
            (Transformation|SetRelativeTransform (Variables|Default|GetCard) (Math|Transform|MakeTransform (Math|Vector|MakeVector 60.180981 -45.260174 23.768196) (Variables|/Script/Engine.SceneComponent|GetRelativeRotation _card) (Variables|/Script/Engine.SceneComponent|GetRelativeScale3D _card)) false false)
            (Utilities|FlowControl|Delay 0.2)
            (bind (_direction _newtrack_x _newtrack_y _newtrack_z) (Timeline|Card%20Swiping PlayFromStart)
              (:Update
                (Transformation|SetRelativeTransform (Variables|Default|GetCard) (Math|Transform|MakeTransform (Math|Vector|MakeVector _newtrack_x _newtrack_y _newtrack_z) (Variables|/Script/Engine.SceneComponent|GetRelativeRotation _card_2) (Variables|/Script/Engine.SceneComponent|GetRelativeScale3D _card_2)) false false))
              (:Finished
                (Utilities|FlowControl|Delay 0.2)
                (Rendering|SetVisibility (Variables|Default|GetCard) false false))))
          (:then_2
            (goto _label Close)))))))

(event Input|KeyboardEvents|NumPadTwo
  (params (Key :type Key%20Structure :default "None"))
  (bind _returnvalue (Game|GetPlayerController 0))
  (bind _returnvalue_2 (Game|GetPlayerController 0))
  (bind _greenbuttons (Variables|Default|GetGreenButtons))
  (bind _greenbuttons_2 (Variables|Default|GetGreenButtons))
  (bind _door (Variables|Default|GetDoor))
  (bind _returnvalue_3 (Transformation|GetWorldLocation _door))
  (:Pressed
    (Variables|Default|SetNumPressed 2)
    (if (not (Variables|Default|GetDoorOpened))
      (if (Variables|Default|GetReadyForPassword)
        (Utilities|FlowControl|Sequence
          (:then_0
            (if (== (Variables|Default|GetPasswordIndex) 0)
              (if (== (Variables|Default|GetNumPressed) (Utilities|Array|Get(acopy) (Variables|Default|GetPassword)))
                (Audio|PlaySound2D "/Game/Game/Sounds/Button/ButtonPush_S011FO_80_Cue.ButtonPush_S011FO_80_Cue" 0.5 1.0 0.0 0 0 :!label _label)
                (Utilities|FlowControl|Sequence
                  (:then_0
                    (if (== (Variables|Default|GetNumPressed) 1)
                      (Utilities|FlowControl|Sequence
                        (:then_0
                          (bind _newtrack_0 (Timeline|Pressing%201 PlayFromStart)
                            (:Update
                              (Transformation|SetRelativeTransform (Variables|Default|GetButton1) (Math|Transform|MakeTransform (Math|Vector|MakeVector 0.0 _newtrack_0 0.0) "0, 0, 0" "1.000000,1.000000,1.000000") false false))))
                        (:then_1
                          (Utilities|FlowControl|Sequence
                            (:then_0
                              (Utilities|FlowControl|Delay 0.2)
                              (Rendering|SetVisibility (Variables|Default|GetTextButton1) false false)
                              (Rendering|SetVisibility (Variables|Default|GetTextButton1Green) true false)
                              (Utilities|Array|SetArrayElem _greenbuttons 0 true))
                            (:then_1
                              (Input|DisableInput _returnvalue_2 :!label _label_2)
                              (Utilities|FlowControl|Delay 0.001)
                              (Variables|Default|SetPasswordIndex (+ (Variables|Default|GetPasswordIndex) 1))
                              (Input|EnableInput _returnvalue_2)))))))
                  (:then_1
                    (if (== (Variables|Default|GetNumPressed) 2)
                      (Utilities|FlowControl|Sequence
                        (:then_0
                          (bind _newtrack_0_2 (Timeline|Pressing%202 PlayFromStart)
                            (:Update
                              (Transformation|SetRelativeTransform (Variables|Default|GetButton2) (Math|Transform|MakeTransform (Math|Vector|MakeVector 123.529412 _newtrack_0_2 0.0) "0, 0, 0" "1.000000,1.000000,1.000000") false false))))
                        (:then_1
                          (Utilities|FlowControl|Sequence
                            (:then_0
                              (Utilities|FlowControl|Delay 0.2)
                              (Rendering|SetVisibility (Variables|Default|GetTextButton2) false false)
                              (Rendering|SetVisibility (Variables|Default|GetTextButton2Green) true false)
                              (Utilities|Array|SetArrayElem _greenbuttons 1 true))
                            (:then_1
                              (goto _label_2)))))))
                  (:then_2
                    (if (== (Variables|Default|GetNumPressed) 3)
                      (Utilities|FlowControl|Sequence
                        (:then_0
                          (bind _newtrack_0_3 (Timeline|Pressing%203 PlayFromStart)
                            (:Update
                              (Transformation|SetRelativeTransform (Variables|Default|GetButton3) (Math|Transform|MakeTransform (Math|Vector|MakeVector 0.0 _newtrack_0_3 -135.294116) "0, 0, 0" "1.000000,1.000000,1.000000") false false))))
                        (:then_1
                          (Utilities|FlowControl|Sequence
                            (:then_0
                              (Utilities|FlowControl|Delay 0.2)
                              (Rendering|SetVisibility (Variables|Default|GetTextButton3) false false)
                              (Rendering|SetVisibility (Variables|Default|GetTextButton3Green) true false)
                              (Utilities|Array|SetArrayElem _greenbuttons_2 2 true))
                            (:then_1
                              (goto _label_2)))))))
                  (:then_3
                    (if (== (Variables|Default|GetNumPressed) 4)
                      (Utilities|FlowControl|Sequence
                        (:then_0
                          (bind _newtrack_0_4 (Timeline|Pressing%204 PlayFromStart)
                            (:Update
                              (Transformation|SetRelativeTransform (Variables|Default|GetButton4) (Math|Transform|MakeTransform (Math|Vector|MakeVector 123.52941 _newtrack_0_4 -135.294116) "0, 0, 0" "1.000000,1.000000,1.000000") false false))))
                        (:then_1
                          (Utilities|FlowControl|Sequence
                            (:then_0
                              (Utilities|FlowControl|Delay 0.2)
                              (Rendering|SetVisibility (Variables|Default|GetTextButton4) false false)
                              (Rendering|SetVisibility (Variables|Default|GetTextButton4Green) true false)
                              (Utilities|Array|SetArrayElem _greenbuttons_2 3 true))
                            (:then_1
                              (goto _label_2))))))))
                (else
                  (Utilities|FlowControl|Sequence :!label _label_3
                    (:then_0
                      (if (== (Variables|Default|GetNumPressed) 1)
                        (if (not (Utilities|Array|Get(acopy) (Variables|Default|GetGreenButtons)))
                          (Utilities|FlowControl|Sequence
                            (:then_0
                              (Timeline|Pressing%201 PlayFromStart))
                            (:then_1
                              (Utilities|FlowControl|Delay 0.2)
                              (Rendering|SetVisibility (Variables|Default|GetTextButton1) false false)
                              (Rendering|SetVisibility (Variables|Default|GetTextButton1Red) true false))
                            (:then_2
                              (Audio|PlaySound2D "/Game/Game/Sounds/Button/ButtonPush_S011FO_80_Cue.ButtonPush_S011FO_80_Cue" 0.5 1.0 0.0 0 0 :!label _label_4)
                              (Input|DisableInput _returnvalue)
                              (Audio|PlaySound2D "/Engine/EditorSounds/Notifications/CompileFailed_Cue.CompileFailed_Cue" 2.0 1.0 0.0 0 0)
                              (Utilities|FlowControl|Delay 0.8)
                              (Input|EnableInput _returnvalue)
                              (Rendering|SetVisibility (Variables|Default|GetTextButton1) true false :!label _label_5)
                              (Rendering|SetVisibility (Variables|Default|GetTextButton1Green) false false)
                              (Variables|Default|SetPasswordIndex 0)
                              (Utilities|FlowControl|Sequence
                                (:then_0
                                  (if (Utilities|Array|Get(acopy) (Variables|Default|GetGreenButtons))
                                    (Timeline|Pressing%201 ReverseFromEnd)
                                    (elif (== (Variables|Default|GetNumPressed) 1)
                                      (Timeline|Pressing%201 ReverseFromEnd)
                                      (else
                                        (Utilities|FlowControl|Delay 0.001 :!label _label_6)
                                        (for (_ _array_index) (Variables|Default|GetGreenButtons)
                                          (Utilities|Array|SetArrayElem (Variables|Default|GetGreenButtons) _array_index false))))))
                                (:then_1
                                  (if (Utilities|Array|Get(acopy) (Variables|Default|GetGreenButtons) 1)
                                    (Timeline|Pressing%202 ReverseFromEnd)
                                    (elif (== (Variables|Default|GetNumPressed) 2)
                                      (Timeline|Pressing%202 ReverseFromEnd)
                                      (else
                                        (goto _label_6)))))
                                (:then_2
                                  (if (Utilities|Array|Get(acopy) (Variables|Default|GetGreenButtons) 2)
                                    (Timeline|Pressing%203 ReverseFromEnd)
                                    (elif (== (Variables|Default|GetNumPressed) 3)
                                      (Timeline|Pressing%203 ReverseFromEnd)
                                      (else
                                        (goto _label_6)))))
                                (:then_3
                                  (if (Utilities|Array|Get(acopy) (Variables|Default|GetGreenButtons) 3)
                                    (Timeline|Pressing%204 ReverseFromEnd)
                                    (elif (== (Variables|Default|GetNumPressed) 4)
                                      (Timeline|Pressing%204 ReverseFromEnd)
                                      (else
                                        (goto _label_6)))))))))))
                    (:then_1
                      (if (== (Variables|Default|GetNumPressed) 2)
                        (if (not (Utilities|Array|Get(acopy) (Variables|Default|GetGreenButtons) 1))
                          (Utilities|FlowControl|Sequence
                            (:then_0
                              (Timeline|Pressing%202 PlayFromStart))
                            (:then_1
                              (Utilities|FlowControl|Delay 0.2)
                              (Rendering|SetVisibility (Variables|Default|GetTextButton2) false false)
                              (Rendering|SetVisibility (Variables|Default|GetTextButton2Red) true false))
                            (:then_2
                              (goto _label_4))))))
                    (:then_2
                      (if (== (Variables|Default|GetNumPressed) 3)
                        (if (not (Utilities|Array|Get(acopy) (Variables|Default|GetGreenButtons) 2))
                          (Utilities|FlowControl|Sequence
                            (:then_0
                              (Timeline|Pressing%203 PlayFromStart))
                            (:then_1
                              (Utilities|FlowControl|Delay 0.2)
                              (Rendering|SetVisibility (Variables|Default|GetTextButton3) false false)
                              (Rendering|SetVisibility (Variables|Default|GetTextButton3Red) true false))
                            (:then_2
                              (goto _label_4))))))
                    (:then_3
                      (if (== (Variables|Default|GetNumPressed) 4)
                        (if (not (Utilities|Array|Get(acopy) (Variables|Default|GetGreenButtons) 3))
                          (Utilities|FlowControl|Sequence
                            (:then_0
                              (Timeline|Pressing%204 PlayFromStart))
                            (:then_1
                              (Utilities|FlowControl|Delay 0.2)
                              (Rendering|SetVisibility (Variables|Default|GetTextButton4) false false)
                              (Rendering|SetVisibility (Variables|Default|GetTextButton4Red) true false))
                            (:then_2
                              (goto _label_4)))))))))))
          (:then_1
            (if (== (Variables|Default|GetPasswordIndex) 1)
              (if (== (Variables|Default|GetNumPressed) (Utilities|Array|Get(acopy) (Variables|Default|GetPassword) 1))
                (goto _label)
                (else
                  (goto _label_3)))))
          (:then_2
            (if (== (Variables|Default|GetPasswordIndex) 2)
              (if (== (Variables|Default|GetNumPressed) (Utilities|Array|Get(acopy) (Variables|Default|GetPassword) 2))
                (goto _label)
                (else
                  (goto _label_3)))))
          (:then_3
            (if (== (Variables|Default|GetPasswordIndex) 3)
              (if (== (Variables|Default|GetNumPressed) (Utilities|Array|Get(acopy) (Variables|Default|GetPassword) 3))
                (Utilities|FlowControl|Sequence
                  (:then_0
                    (goto _label))
                  (:then_1
                    (Utilities|FlowControl|Gate true
                      (:Exit
                        (Utilities|FlowControl|Delay 0.2)
                        (Rendering|SetVisibility (Variables|Default|GetBlueScreen) false false)
                        (Rendering|SetVisibility (Variables|Default|GetGreenScreen) true false)
                        (Widget|RemovefromParent (stale OnComponentBeginOverlap(Trigger) _returnvalue_2))
                        (Variables|Default|SetDoorOpened true)
                        (Audio|PlaySound2D "/Engine/VREditor/Sounds/UI/Click_on_Button_Cue.Click_on_Button_Cue" 2.0 1.0 0.0 0 0)
                        (Audio|PlaySoundatLocation "/Game/Maps/AMalginov/BluePrints/Sound_Lock-Click.Sound_Lock-Click" _returnvalue_3 "0, 0, 0" 0.2 1.0 0.0 0 0 0 0)
                        (Utilities|FlowControl|Sequence
                          (:then_0
                            (Utilities|FlowControl|Delay 1.0)
                            (bind _newtrack_0_5 (Timeline|Door%20Rotation Play)
                              (:Update
                                (Transformation|SetRelativeRotation (Variables|Default|GetDoor) (Math|Rotator|MakeRotator 0.0 0.0 _newtrack_0_5) false false))))
                          (:then_1
                            (Utilities|FlowControl|Delay 0.6)
                            (Audio|PlaySoundatLocation "/Game/Maps/AMalginov/BluePrints/Sound_Opening-of-a-big-rusty-metal-door.Sound_Opening-of-a-big-rusty-metal-door" _returnvalue_3 "0, 0, 0" 0.5 1.0 0.0 0 0 0 0)))
                        (Utilities|FlowControl|Delay 4.0)
                        (goto _label_5)))))
                (else
                  (goto _label_3))))))))))

(event Input|KeyboardEvents|NumPadOne
  (params (Key :type Key%20Structure :default "None"))
  (bind _returnvalue (Game|GetPlayerController 0))
  (bind _returnvalue_2 (Game|GetPlayerController 0))
  (bind _greenbuttons (Variables|Default|GetGreenButtons))
  (bind _greenbuttons_2 (Variables|Default|GetGreenButtons))
  (bind _door (Variables|Default|GetDoor))
  (bind _returnvalue_3 (Transformation|GetWorldLocation _door))
  (:Pressed
    (Variables|Default|SetNumPressed 1)
    (if (not (Variables|Default|GetDoorOpened))
      (if (Variables|Default|GetReadyForPassword)
        (Utilities|FlowControl|Sequence
          (:then_0
            (if (== (Variables|Default|GetPasswordIndex) 0)
              (if (== (Variables|Default|GetNumPressed) (Utilities|Array|Get(acopy) (Variables|Default|GetPassword)))
                (Audio|PlaySound2D "/Game/Game/Sounds/Button/ButtonPush_S011FO_80_Cue.ButtonPush_S011FO_80_Cue" 0.5 1.0 0.0 0 0 :!label _label)
                (Utilities|FlowControl|Sequence
                  (:then_0
                    (if (== (Variables|Default|GetNumPressed) 1)
                      (Utilities|FlowControl|Sequence
                        (:then_0
                          (bind _newtrack_0 (Timeline|Pressing%201 PlayFromStart)
                            (:Update
                              (Transformation|SetRelativeTransform (Variables|Default|GetButton1) (Math|Transform|MakeTransform (Math|Vector|MakeVector 0.0 _newtrack_0 0.0) "0, 0, 0" "1.000000,1.000000,1.000000") false false))))
                        (:then_1
                          (Utilities|FlowControl|Sequence
                            (:then_0
                              (Utilities|FlowControl|Delay 0.2)
                              (Rendering|SetVisibility (Variables|Default|GetTextButton1) false false)
                              (Rendering|SetVisibility (Variables|Default|GetTextButton1Green) true false)
                              (Utilities|Array|SetArrayElem _greenbuttons 0 true))
                            (:then_1
                              (Input|DisableInput _returnvalue_2 :!label _label_2)
                              (Utilities|FlowControl|Delay 0.001)
                              (Variables|Default|SetPasswordIndex (+ (Variables|Default|GetPasswordIndex) 1))
                              (Input|EnableInput _returnvalue_2)))))))
                  (:then_1
                    (if (== (Variables|Default|GetNumPressed) 2)
                      (Utilities|FlowControl|Sequence
                        (:then_0
                          (bind _newtrack_0_2 (Timeline|Pressing%202 PlayFromStart)
                            (:Update
                              (Transformation|SetRelativeTransform (Variables|Default|GetButton2) (Math|Transform|MakeTransform (Math|Vector|MakeVector 123.529412 _newtrack_0_2 0.0) "0, 0, 0" "1.000000,1.000000,1.000000") false false))))
                        (:then_1
                          (Utilities|FlowControl|Sequence
                            (:then_0
                              (Utilities|FlowControl|Delay 0.2)
                              (Rendering|SetVisibility (Variables|Default|GetTextButton2) false false)
                              (Rendering|SetVisibility (Variables|Default|GetTextButton2Green) true false)
                              (Utilities|Array|SetArrayElem _greenbuttons 1 true))
                            (:then_1
                              (goto _label_2)))))))
                  (:then_2
                    (if (== (Variables|Default|GetNumPressed) 3)
                      (Utilities|FlowControl|Sequence
                        (:then_0
                          (bind _newtrack_0_3 (Timeline|Pressing%203 PlayFromStart)
                            (:Update
                              (Transformation|SetRelativeTransform (Variables|Default|GetButton3) (Math|Transform|MakeTransform (Math|Vector|MakeVector 0.0 _newtrack_0_3 -135.294116) "0, 0, 0" "1.000000,1.000000,1.000000") false false))))
                        (:then_1
                          (Utilities|FlowControl|Sequence
                            (:then_0
                              (Utilities|FlowControl|Delay 0.2)
                              (Rendering|SetVisibility (Variables|Default|GetTextButton3) false false)
                              (Rendering|SetVisibility (Variables|Default|GetTextButton3Green) true false)
                              (Utilities|Array|SetArrayElem _greenbuttons_2 2 true))
                            (:then_1
                              (goto _label_2)))))))
                  (:then_3
                    (if (== (Variables|Default|GetNumPressed) 4)
                      (Utilities|FlowControl|Sequence
                        (:then_0
                          (bind _newtrack_0_4 (Timeline|Pressing%204 PlayFromStart)
                            (:Update
                              (Transformation|SetRelativeTransform (Variables|Default|GetButton4) (Math|Transform|MakeTransform (Math|Vector|MakeVector 123.52941 _newtrack_0_4 -135.294116) "0, 0, 0" "1.000000,1.000000,1.000000") false false))))
                        (:then_1
                          (Utilities|FlowControl|Sequence
                            (:then_0
                              (Utilities|FlowControl|Delay 0.2)
                              (Rendering|SetVisibility (Variables|Default|GetTextButton4) false false)
                              (Rendering|SetVisibility (Variables|Default|GetTextButton4Green) true false)
                              (Utilities|Array|SetArrayElem _greenbuttons_2 3 true))
                            (:then_1
                              (goto _label_2))))))))
                (else
                  (Utilities|FlowControl|Sequence :!label _label_3
                    (:then_0
                      (if (== (Variables|Default|GetNumPressed) 1)
                        (if (not (Utilities|Array|Get(acopy) (Variables|Default|GetGreenButtons)))
                          (Utilities|FlowControl|Sequence
                            (:then_0
                              (Timeline|Pressing%201 PlayFromStart))
                            (:then_1
                              (Utilities|FlowControl|Delay 0.2)
                              (Rendering|SetVisibility (Variables|Default|GetTextButton1) false false)
                              (Rendering|SetVisibility (Variables|Default|GetTextButton1Red) true false))
                            (:then_2
                              (Audio|PlaySound2D "/Game/Game/Sounds/Button/ButtonPush_S011FO_80_Cue.ButtonPush_S011FO_80_Cue" 0.5 1.0 0.0 0 0 :!label _label_4)
                              (Input|DisableInput _returnvalue)
                              (Audio|PlaySound2D "/Engine/EditorSounds/Notifications/CompileFailed_Cue.CompileFailed_Cue" 2.0 1.0 0.0 0 0)
                              (Utilities|FlowControl|Delay 0.8)
                              (Input|EnableInput _returnvalue)
                              (Rendering|SetVisibility (Variables|Default|GetTextButton1) true false :!label _label_5)
                              (Rendering|SetVisibility (Variables|Default|GetTextButton1Green) false false)
                              (Variables|Default|SetPasswordIndex 0)
                              (Utilities|FlowControl|Sequence
                                (:then_0
                                  (if (Utilities|Array|Get(acopy) (Variables|Default|GetGreenButtons))
                                    (Timeline|Pressing%201 ReverseFromEnd)
                                    (elif (== (Variables|Default|GetNumPressed) 1)
                                      (Timeline|Pressing%201 ReverseFromEnd)
                                      (else
                                        (Utilities|FlowControl|Delay 0.001 :!label _label_6)
                                        (for (_ _array_index) (Variables|Default|GetGreenButtons)
                                          (Utilities|Array|SetArrayElem (Variables|Default|GetGreenButtons) _array_index false))))))
                                (:then_1
                                  (if (Utilities|Array|Get(acopy) (Variables|Default|GetGreenButtons) 1)
                                    (Timeline|Pressing%202 ReverseFromEnd)
                                    (elif (== (Variables|Default|GetNumPressed) 2)
                                      (Timeline|Pressing%202 ReverseFromEnd)
                                      (else
                                        (goto _label_6)))))
                                (:then_2
                                  (if (Utilities|Array|Get(acopy) (Variables|Default|GetGreenButtons) 2)
                                    (Timeline|Pressing%203 ReverseFromEnd)
                                    (elif (== (Variables|Default|GetNumPressed) 3)
                                      (Timeline|Pressing%203 ReverseFromEnd)
                                      (else
                                        (goto _label_6)))))
                                (:then_3
                                  (if (Utilities|Array|Get(acopy) (Variables|Default|GetGreenButtons) 3)
                                    (Timeline|Pressing%204 ReverseFromEnd)
                                    (elif (== (Variables|Default|GetNumPressed) 4)
                                      (Timeline|Pressing%204 ReverseFromEnd)
                                      (else
                                        (goto _label_6)))))))))))
                    (:then_1
                      (if (== (Variables|Default|GetNumPressed) 2)
                        (if (not (Utilities|Array|Get(acopy) (Variables|Default|GetGreenButtons) 1))
                          (Utilities|FlowControl|Sequence
                            (:then_0
                              (Timeline|Pressing%202 PlayFromStart))
                            (:then_1
                              (Utilities|FlowControl|Delay 0.2)
                              (Rendering|SetVisibility (Variables|Default|GetTextButton2) false false)
                              (Rendering|SetVisibility (Variables|Default|GetTextButton2Red) true false))
                            (:then_2
                              (goto _label_4))))))
                    (:then_2
                      (if (== (Variables|Default|GetNumPressed) 3)
                        (if (not (Utilities|Array|Get(acopy) (Variables|Default|GetGreenButtons) 2))
                          (Utilities|FlowControl|Sequence
                            (:then_0
                              (Timeline|Pressing%203 PlayFromStart))
                            (:then_1
                              (Utilities|FlowControl|Delay 0.2)
                              (Rendering|SetVisibility (Variables|Default|GetTextButton3) false false)
                              (Rendering|SetVisibility (Variables|Default|GetTextButton3Red) true false))
                            (:then_2
                              (goto _label_4))))))
                    (:then_3
                      (if (== (Variables|Default|GetNumPressed) 4)
                        (if (not (Utilities|Array|Get(acopy) (Variables|Default|GetGreenButtons) 3))
                          (Utilities|FlowControl|Sequence
                            (:then_0
                              (Timeline|Pressing%204 PlayFromStart))
                            (:then_1
                              (Utilities|FlowControl|Delay 0.2)
                              (Rendering|SetVisibility (Variables|Default|GetTextButton4) false false)
                              (Rendering|SetVisibility (Variables|Default|GetTextButton4Red) true false))
                            (:then_2
                              (goto _label_4)))))))))))
          (:then_1
            (if (== (Variables|Default|GetPasswordIndex) 1)
              (if (== (Variables|Default|GetNumPressed) (Utilities|Array|Get(acopy) (Variables|Default|GetPassword) 1))
                (goto _label)
                (else
                  (goto _label_3)))))
          (:then_2
            (if (== (Variables|Default|GetPasswordIndex) 2)
              (if (== (Variables|Default|GetNumPressed) (Utilities|Array|Get(acopy) (Variables|Default|GetPassword) 2))
                (goto _label)
                (else
                  (goto _label_3)))))
          (:then_3
            (if (== (Variables|Default|GetPasswordIndex) 3)
              (if (== (Variables|Default|GetNumPressed) (Utilities|Array|Get(acopy) (Variables|Default|GetPassword) 3))
                (Utilities|FlowControl|Sequence
                  (:then_0
                    (goto _label))
                  (:then_1
                    (Utilities|FlowControl|Gate true
                      (:Exit
                        (Utilities|FlowControl|Delay 0.2)
                        (Rendering|SetVisibility (Variables|Default|GetBlueScreen) false false)
                        (Rendering|SetVisibility (Variables|Default|GetGreenScreen) true false)
                        (Widget|RemovefromParent (stale OnComponentBeginOverlap(Trigger) _returnvalue_2))
                        (Variables|Default|SetDoorOpened true)
                        (Audio|PlaySound2D "/Engine/VREditor/Sounds/UI/Click_on_Button_Cue.Click_on_Button_Cue" 2.0 1.0 0.0 0 0)
                        (Audio|PlaySoundatLocation "/Game/Maps/AMalginov/BluePrints/Sound_Lock-Click.Sound_Lock-Click" _returnvalue_3 "0, 0, 0" 0.2 1.0 0.0 0 0 0 0)
                        (Utilities|FlowControl|Sequence
                          (:then_0
                            (Utilities|FlowControl|Delay 1.0)
                            (bind _newtrack_0_5 (Timeline|Door%20Rotation Play)
                              (:Update
                                (Transformation|SetRelativeRotation (Variables|Default|GetDoor) (Math|Rotator|MakeRotator 0.0 0.0 _newtrack_0_5) false false))))
                          (:then_1
                            (Utilities|FlowControl|Delay 0.6)
                            (Audio|PlaySoundatLocation "/Game/Maps/AMalginov/BluePrints/Sound_Opening-of-a-big-rusty-metal-door.Sound_Opening-of-a-big-rusty-metal-door" _returnvalue_3 "0, 0, 0" 0.5 1.0 0.0 0 0 0 0)))
                        (Utilities|FlowControl|Delay 4.0)
                        (goto _label_5)))))
                (else
                  (goto _label_3))))))))))

(event Input|KeyboardEvents|NumPadThree
  (params (Key :type Key%20Structure :default "None"))
  (bind _returnvalue (Game|GetPlayerController 0))
  (bind _returnvalue_2 (Game|GetPlayerController 0))
  (bind _greenbuttons (Variables|Default|GetGreenButtons))
  (bind _greenbuttons_2 (Variables|Default|GetGreenButtons))
  (bind _door (Variables|Default|GetDoor))
  (bind _returnvalue_3 (Transformation|GetWorldLocation _door))
  (:Pressed
    (Variables|Default|SetNumPressed 3)
    (if (not (Variables|Default|GetDoorOpened))
      (if (Variables|Default|GetReadyForPassword)
        (Utilities|FlowControl|Sequence
          (:then_0
            (if (== (Variables|Default|GetPasswordIndex) 0)
              (if (== (Variables|Default|GetNumPressed) (Utilities|Array|Get(acopy) (Variables|Default|GetPassword)))
                (Audio|PlaySound2D "/Game/Game/Sounds/Button/ButtonPush_S011FO_80_Cue.ButtonPush_S011FO_80_Cue" 0.5 1.0 0.0 0 0 :!label _label)
                (Utilities|FlowControl|Sequence
                  (:then_0
                    (if (== (Variables|Default|GetNumPressed) 1)
                      (Utilities|FlowControl|Sequence
                        (:then_0
                          (bind _newtrack_0 (Timeline|Pressing%201 PlayFromStart)
                            (:Update
                              (Transformation|SetRelativeTransform (Variables|Default|GetButton1) (Math|Transform|MakeTransform (Math|Vector|MakeVector 0.0 _newtrack_0 0.0) "0, 0, 0" "1.000000,1.000000,1.000000") false false))))
                        (:then_1
                          (Utilities|FlowControl|Sequence
                            (:then_0
                              (Utilities|FlowControl|Delay 0.2)
                              (Rendering|SetVisibility (Variables|Default|GetTextButton1) false false)
                              (Rendering|SetVisibility (Variables|Default|GetTextButton1Green) true false)
                              (Utilities|Array|SetArrayElem _greenbuttons 0 true))
                            (:then_1
                              (Input|DisableInput _returnvalue_2 :!label _label_2)
                              (Utilities|FlowControl|Delay 0.001)
                              (Variables|Default|SetPasswordIndex (+ (Variables|Default|GetPasswordIndex) 1))
                              (Input|EnableInput _returnvalue_2)))))))
                  (:then_1
                    (if (== (Variables|Default|GetNumPressed) 2)
                      (Utilities|FlowControl|Sequence
                        (:then_0
                          (bind _newtrack_0_2 (Timeline|Pressing%202 PlayFromStart)
                            (:Update
                              (Transformation|SetRelativeTransform (Variables|Default|GetButton2) (Math|Transform|MakeTransform (Math|Vector|MakeVector 123.529412 _newtrack_0_2 0.0) "0, 0, 0" "1.000000,1.000000,1.000000") false false))))
                        (:then_1
                          (Utilities|FlowControl|Sequence
                            (:then_0
                              (Utilities|FlowControl|Delay 0.2)
                              (Rendering|SetVisibility (Variables|Default|GetTextButton2) false false)
                              (Rendering|SetVisibility (Variables|Default|GetTextButton2Green) true false)
                              (Utilities|Array|SetArrayElem _greenbuttons 1 true))
                            (:then_1
                              (goto _label_2)))))))
                  (:then_2
                    (if (== (Variables|Default|GetNumPressed) 3)
                      (Utilities|FlowControl|Sequence
                        (:then_0
                          (bind _newtrack_0_3 (Timeline|Pressing%203 PlayFromStart)
                            (:Update
                              (Transformation|SetRelativeTransform (Variables|Default|GetButton3) (Math|Transform|MakeTransform (Math|Vector|MakeVector 0.0 _newtrack_0_3 -135.294116) "0, 0, 0" "1.000000,1.000000,1.000000") false false))))
                        (:then_1
                          (Utilities|FlowControl|Sequence
                            (:then_0
                              (Utilities|FlowControl|Delay 0.2)
                              (Rendering|SetVisibility (Variables|Default|GetTextButton3) false false)
                              (Rendering|SetVisibility (Variables|Default|GetTextButton3Green) true false)
                              (Utilities|Array|SetArrayElem _greenbuttons_2 2 true))
                            (:then_1
                              (goto _label_2)))))))
                  (:then_3
                    (if (== (Variables|Default|GetNumPressed) 4)
                      (Utilities|FlowControl|Sequence
                        (:then_0
                          (bind _newtrack_0_4 (Timeline|Pressing%204 PlayFromStart)
                            (:Update
                              (Transformation|SetRelativeTransform (Variables|Default|GetButton4) (Math|Transform|MakeTransform (Math|Vector|MakeVector 123.52941 _newtrack_0_4 -135.294116) "0, 0, 0" "1.000000,1.000000,1.000000") false false))))
                        (:then_1
                          (Utilities|FlowControl|Sequence
                            (:then_0
                              (Utilities|FlowControl|Delay 0.2)
                              (Rendering|SetVisibility (Variables|Default|GetTextButton4) false false)
                              (Rendering|SetVisibility (Variables|Default|GetTextButton4Green) true false)
                              (Utilities|Array|SetArrayElem _greenbuttons_2 3 true))
                            (:then_1
                              (goto _label_2))))))))
                (else
                  (Utilities|FlowControl|Sequence :!label _label_3
                    (:then_0
                      (if (== (Variables|Default|GetNumPressed) 1)
                        (if (not (Utilities|Array|Get(acopy) (Variables|Default|GetGreenButtons)))
                          (Utilities|FlowControl|Sequence
                            (:then_0
                              (Timeline|Pressing%201 PlayFromStart))
                            (:then_1
                              (Utilities|FlowControl|Delay 0.2)
                              (Rendering|SetVisibility (Variables|Default|GetTextButton1) false false)
                              (Rendering|SetVisibility (Variables|Default|GetTextButton1Red) true false))
                            (:then_2
                              (Audio|PlaySound2D "/Game/Game/Sounds/Button/ButtonPush_S011FO_80_Cue.ButtonPush_S011FO_80_Cue" 0.5 1.0 0.0 0 0 :!label _label_4)
                              (Input|DisableInput _returnvalue)
                              (Audio|PlaySound2D "/Engine/EditorSounds/Notifications/CompileFailed_Cue.CompileFailed_Cue" 2.0 1.0 0.0 0 0)
                              (Utilities|FlowControl|Delay 0.8)
                              (Input|EnableInput _returnvalue)
                              (Rendering|SetVisibility (Variables|Default|GetTextButton1) true false :!label _label_5)
                              (Rendering|SetVisibility (Variables|Default|GetTextButton1Green) false false)
                              (Variables|Default|SetPasswordIndex 0)
                              (Utilities|FlowControl|Sequence
                                (:then_0
                                  (if (Utilities|Array|Get(acopy) (Variables|Default|GetGreenButtons))
                                    (Timeline|Pressing%201 ReverseFromEnd)
                                    (elif (== (Variables|Default|GetNumPressed) 1)
                                      (Timeline|Pressing%201 ReverseFromEnd)
                                      (else
                                        (Utilities|FlowControl|Delay 0.001 :!label _label_6)
                                        (for (_ _array_index) (Variables|Default|GetGreenButtons)
                                          (Utilities|Array|SetArrayElem (Variables|Default|GetGreenButtons) _array_index false))))))
                                (:then_1
                                  (if (Utilities|Array|Get(acopy) (Variables|Default|GetGreenButtons) 1)
                                    (Timeline|Pressing%202 ReverseFromEnd)
                                    (elif (== (Variables|Default|GetNumPressed) 2)
                                      (Timeline|Pressing%202 ReverseFromEnd)
                                      (else
                                        (goto _label_6)))))
                                (:then_2
                                  (if (Utilities|Array|Get(acopy) (Variables|Default|GetGreenButtons) 2)
                                    (Timeline|Pressing%203 ReverseFromEnd)
                                    (elif (== (Variables|Default|GetNumPressed) 3)
                                      (Timeline|Pressing%203 ReverseFromEnd)
                                      (else
                                        (goto _label_6)))))
                                (:then_3
                                  (if (Utilities|Array|Get(acopy) (Variables|Default|GetGreenButtons) 3)
                                    (Timeline|Pressing%204 ReverseFromEnd)
                                    (elif (== (Variables|Default|GetNumPressed) 4)
                                      (Timeline|Pressing%204 ReverseFromEnd)
                                      (else
                                        (goto _label_6)))))))))))
                    (:then_1
                      (if (== (Variables|Default|GetNumPressed) 2)
                        (if (not (Utilities|Array|Get(acopy) (Variables|Default|GetGreenButtons) 1))
                          (Utilities|FlowControl|Sequence
                            (:then_0
                              (Timeline|Pressing%202 PlayFromStart))
                            (:then_1
                              (Utilities|FlowControl|Delay 0.2)
                              (Rendering|SetVisibility (Variables|Default|GetTextButton2) false false)
                              (Rendering|SetVisibility (Variables|Default|GetTextButton2Red) true false))
                            (:then_2
                              (goto _label_4))))))
                    (:then_2
                      (if (== (Variables|Default|GetNumPressed) 3)
                        (if (not (Utilities|Array|Get(acopy) (Variables|Default|GetGreenButtons) 2))
                          (Utilities|FlowControl|Sequence
                            (:then_0
                              (Timeline|Pressing%203 PlayFromStart))
                            (:then_1
                              (Utilities|FlowControl|Delay 0.2)
                              (Rendering|SetVisibility (Variables|Default|GetTextButton3) false false)
                              (Rendering|SetVisibility (Variables|Default|GetTextButton3Red) true false))
                            (:then_2
                              (goto _label_4))))))
                    (:then_3
                      (if (== (Variables|Default|GetNumPressed) 4)
                        (if (not (Utilities|Array|Get(acopy) (Variables|Default|GetGreenButtons) 3))
                          (Utilities|FlowControl|Sequence
                            (:then_0
                              (Timeline|Pressing%204 PlayFromStart))
                            (:then_1
                              (Utilities|FlowControl|Delay 0.2)
                              (Rendering|SetVisibility (Variables|Default|GetTextButton4) false false)
                              (Rendering|SetVisibility (Variables|Default|GetTextButton4Red) true false))
                            (:then_2
                              (goto _label_4)))))))))))
          (:then_1
            (if (== (Variables|Default|GetPasswordIndex) 1)
              (if (== (Variables|Default|GetNumPressed) (Utilities|Array|Get(acopy) (Variables|Default|GetPassword) 1))
                (goto _label)
                (else
                  (goto _label_3)))))
          (:then_2
            (if (== (Variables|Default|GetPasswordIndex) 2)
              (if (== (Variables|Default|GetNumPressed) (Utilities|Array|Get(acopy) (Variables|Default|GetPassword) 2))
                (goto _label)
                (else
                  (goto _label_3)))))
          (:then_3
            (if (== (Variables|Default|GetPasswordIndex) 3)
              (if (== (Variables|Default|GetNumPressed) (Utilities|Array|Get(acopy) (Variables|Default|GetPassword) 3))
                (Utilities|FlowControl|Sequence
                  (:then_0
                    (goto _label))
                  (:then_1
                    (Utilities|FlowControl|Gate true
                      (:Exit
                        (Utilities|FlowControl|Delay 0.2)
                        (Rendering|SetVisibility (Variables|Default|GetBlueScreen) false false)
                        (Rendering|SetVisibility (Variables|Default|GetGreenScreen) true false)
                        (Widget|RemovefromParent (stale OnComponentBeginOverlap(Trigger) _returnvalue_2))
                        (Variables|Default|SetDoorOpened true)
                        (Audio|PlaySound2D "/Engine/VREditor/Sounds/UI/Click_on_Button_Cue.Click_on_Button_Cue" 2.0 1.0 0.0 0 0)
                        (Audio|PlaySoundatLocation "/Game/Maps/AMalginov/BluePrints/Sound_Lock-Click.Sound_Lock-Click" _returnvalue_3 "0, 0, 0" 0.2 1.0 0.0 0 0 0 0)
                        (Utilities|FlowControl|Sequence
                          (:then_0
                            (Utilities|FlowControl|Delay 1.0)
                            (bind _newtrack_0_5 (Timeline|Door%20Rotation Play)
                              (:Update
                                (Transformation|SetRelativeRotation (Variables|Default|GetDoor) (Math|Rotator|MakeRotator 0.0 0.0 _newtrack_0_5) false false))))
                          (:then_1
                            (Utilities|FlowControl|Delay 0.6)
                            (Audio|PlaySoundatLocation "/Game/Maps/AMalginov/BluePrints/Sound_Opening-of-a-big-rusty-metal-door.Sound_Opening-of-a-big-rusty-metal-door" _returnvalue_3 "0, 0, 0" 0.5 1.0 0.0 0 0 0 0)))
                        (Utilities|FlowControl|Delay 4.0)
                        (goto _label_5)))))
                (else
                  (goto _label_3))))))))))

(event Input|KeyboardEvents|NumPadFour
  (params (Key :type Key%20Structure :default "None"))
  (bind _returnvalue (Game|GetPlayerController 0))
  (bind _returnvalue_2 (Game|GetPlayerController 0))
  (bind _greenbuttons (Variables|Default|GetGreenButtons))
  (bind _greenbuttons_2 (Variables|Default|GetGreenButtons))
  (bind _door (Variables|Default|GetDoor))
  (bind _returnvalue_3 (Transformation|GetWorldLocation _door))
  (:Pressed
    (Variables|Default|SetNumPressed 4)
    (if (not (Variables|Default|GetDoorOpened))
      (if (Variables|Default|GetReadyForPassword)
        (Utilities|FlowControl|Sequence
          (:then_0
            (if (== (Variables|Default|GetPasswordIndex) 0)
              (if (== (Variables|Default|GetNumPressed) (Utilities|Array|Get(acopy) (Variables|Default|GetPassword)))
                (Audio|PlaySound2D "/Game/Game/Sounds/Button/ButtonPush_S011FO_80_Cue.ButtonPush_S011FO_80_Cue" 0.5 1.0 0.0 0 0 :!label _label)
                (Utilities|FlowControl|Sequence
                  (:then_0
                    (if (== (Variables|Default|GetNumPressed) 1)
                      (Utilities|FlowControl|Sequence
                        (:then_0
                          (bind _newtrack_0 (Timeline|Pressing%201 PlayFromStart)
                            (:Update
                              (Transformation|SetRelativeTransform (Variables|Default|GetButton1) (Math|Transform|MakeTransform (Math|Vector|MakeVector 0.0 _newtrack_0 0.0) "0, 0, 0" "1.000000,1.000000,1.000000") false false))))
                        (:then_1
                          (Utilities|FlowControl|Sequence
                            (:then_0
                              (Utilities|FlowControl|Delay 0.2)
                              (Rendering|SetVisibility (Variables|Default|GetTextButton1) false false)
                              (Rendering|SetVisibility (Variables|Default|GetTextButton1Green) true false)
                              (Utilities|Array|SetArrayElem _greenbuttons 0 true))
                            (:then_1
                              (Input|DisableInput _returnvalue_2 :!label _label_2)
                              (Utilities|FlowControl|Delay 0.001)
                              (Variables|Default|SetPasswordIndex (+ (Variables|Default|GetPasswordIndex) 1))
                              (Input|EnableInput _returnvalue_2)))))))
                  (:then_1
                    (if (== (Variables|Default|GetNumPressed) 2)
                      (Utilities|FlowControl|Sequence
                        (:then_0
                          (bind _newtrack_0_2 (Timeline|Pressing%202 PlayFromStart)
                            (:Update
                              (Transformation|SetRelativeTransform (Variables|Default|GetButton2) (Math|Transform|MakeTransform (Math|Vector|MakeVector 123.529412 _newtrack_0_2 0.0) "0, 0, 0" "1.000000,1.000000,1.000000") false false))))
                        (:then_1
                          (Utilities|FlowControl|Sequence
                            (:then_0
                              (Utilities|FlowControl|Delay 0.2)
                              (Rendering|SetVisibility (Variables|Default|GetTextButton2) false false)
                              (Rendering|SetVisibility (Variables|Default|GetTextButton2Green) true false)
                              (Utilities|Array|SetArrayElem _greenbuttons 1 true))
                            (:then_1
                              (goto _label_2)))))))
                  (:then_2
                    (if (== (Variables|Default|GetNumPressed) 3)
                      (Utilities|FlowControl|Sequence
                        (:then_0
                          (bind _newtrack_0_3 (Timeline|Pressing%203 PlayFromStart)
                            (:Update
                              (Transformation|SetRelativeTransform (Variables|Default|GetButton3) (Math|Transform|MakeTransform (Math|Vector|MakeVector 0.0 _newtrack_0_3 -135.294116) "0, 0, 0" "1.000000,1.000000,1.000000") false false))))
                        (:then_1
                          (Utilities|FlowControl|Sequence
                            (:then_0
                              (Utilities|FlowControl|Delay 0.2)
                              (Rendering|SetVisibility (Variables|Default|GetTextButton3) false false)
                              (Rendering|SetVisibility (Variables|Default|GetTextButton3Green) true false)
                              (Utilities|Array|SetArrayElem _greenbuttons_2 2 true))
                            (:then_1
                              (goto _label_2)))))))
                  (:then_3
                    (if (== (Variables|Default|GetNumPressed) 4)
                      (Utilities|FlowControl|Sequence
                        (:then_0
                          (bind _newtrack_0_4 (Timeline|Pressing%204 PlayFromStart)
                            (:Update
                              (Transformation|SetRelativeTransform (Variables|Default|GetButton4) (Math|Transform|MakeTransform (Math|Vector|MakeVector 123.52941 _newtrack_0_4 -135.294116) "0, 0, 0" "1.000000,1.000000,1.000000") false false))))
                        (:then_1
                          (Utilities|FlowControl|Sequence
                            (:then_0
                              (Utilities|FlowControl|Delay 0.2)
                              (Rendering|SetVisibility (Variables|Default|GetTextButton4) false false)
                              (Rendering|SetVisibility (Variables|Default|GetTextButton4Green) true false)
                              (Utilities|Array|SetArrayElem _greenbuttons_2 3 true))
                            (:then_1
                              (goto _label_2))))))))
                (else
                  (Utilities|FlowControl|Sequence :!label _label_3
                    (:then_0
                      (if (== (Variables|Default|GetNumPressed) 1)
                        (if (not (Utilities|Array|Get(acopy) (Variables|Default|GetGreenButtons)))
                          (Utilities|FlowControl|Sequence
                            (:then_0
                              (Timeline|Pressing%201 PlayFromStart))
                            (:then_1
                              (Utilities|FlowControl|Delay 0.2)
                              (Rendering|SetVisibility (Variables|Default|GetTextButton1) false false)
                              (Rendering|SetVisibility (Variables|Default|GetTextButton1Red) true false))
                            (:then_2
                              (Audio|PlaySound2D "/Game/Game/Sounds/Button/ButtonPush_S011FO_80_Cue.ButtonPush_S011FO_80_Cue" 0.5 1.0 0.0 0 0 :!label _label_4)
                              (Input|DisableInput _returnvalue)
                              (Audio|PlaySound2D "/Engine/EditorSounds/Notifications/CompileFailed_Cue.CompileFailed_Cue" 2.0 1.0 0.0 0 0)
                              (Utilities|FlowControl|Delay 0.8)
                              (Input|EnableInput _returnvalue)
                              (Rendering|SetVisibility (Variables|Default|GetTextButton1) true false :!label _label_5)
                              (Rendering|SetVisibility (Variables|Default|GetTextButton1Green) false false)
                              (Variables|Default|SetPasswordIndex 0)
                              (Utilities|FlowControl|Sequence
                                (:then_0
                                  (if (Utilities|Array|Get(acopy) (Variables|Default|GetGreenButtons))
                                    (Timeline|Pressing%201 ReverseFromEnd)
                                    (elif (== (Variables|Default|GetNumPressed) 1)
                                      (Timeline|Pressing%201 ReverseFromEnd)
                                      (else
                                        (Utilities|FlowControl|Delay 0.001 :!label _label_6)
                                        (for (_ _array_index) (Variables|Default|GetGreenButtons)
                                          (Utilities|Array|SetArrayElem (Variables|Default|GetGreenButtons) _array_index false))))))
                                (:then_1
                                  (if (Utilities|Array|Get(acopy) (Variables|Default|GetGreenButtons) 1)
                                    (Timeline|Pressing%202 ReverseFromEnd)
                                    (elif (== (Variables|Default|GetNumPressed) 2)
                                      (Timeline|Pressing%202 ReverseFromEnd)
                                      (else
                                        (goto _label_6)))))
                                (:then_2
                                  (if (Utilities|Array|Get(acopy) (Variables|Default|GetGreenButtons) 2)
                                    (Timeline|Pressing%203 ReverseFromEnd)
                                    (elif (== (Variables|Default|GetNumPressed) 3)
                                      (Timeline|Pressing%203 ReverseFromEnd)
                                      (else
                                        (goto _label_6)))))
                                (:then_3
                                  (if (Utilities|Array|Get(acopy) (Variables|Default|GetGreenButtons) 3)
                                    (Timeline|Pressing%204 ReverseFromEnd)
                                    (elif (== (Variables|Default|GetNumPressed) 4)
                                      (Timeline|Pressing%204 ReverseFromEnd)
                                      (else
                                        (goto _label_6)))))))))))
                    (:then_1
                      (if (== (Variables|Default|GetNumPressed) 2)
                        (if (not (Utilities|Array|Get(acopy) (Variables|Default|GetGreenButtons) 1))
                          (Utilities|FlowControl|Sequence
                            (:then_0
                              (Timeline|Pressing%202 PlayFromStart))
                            (:then_1
                              (Utilities|FlowControl|Delay 0.2)
                              (Rendering|SetVisibility (Variables|Default|GetTextButton2) false false)
                              (Rendering|SetVisibility (Variables|Default|GetTextButton2Red) true false))
                            (:then_2
                              (goto _label_4))))))
                    (:then_2
                      (if (== (Variables|Default|GetNumPressed) 3)
                        (if (not (Utilities|Array|Get(acopy) (Variables|Default|GetGreenButtons) 2))
                          (Utilities|FlowControl|Sequence
                            (:then_0
                              (Timeline|Pressing%203 PlayFromStart))
                            (:then_1
                              (Utilities|FlowControl|Delay 0.2)
                              (Rendering|SetVisibility (Variables|Default|GetTextButton3) false false)
                              (Rendering|SetVisibility (Variables|Default|GetTextButton3Red) true false))
                            (:then_2
                              (goto _label_4))))))
                    (:then_3
                      (if (== (Variables|Default|GetNumPressed) 4)
                        (if (not (Utilities|Array|Get(acopy) (Variables|Default|GetGreenButtons) 3))
                          (Utilities|FlowControl|Sequence
                            (:then_0
                              (Timeline|Pressing%204 PlayFromStart))
                            (:then_1
                              (Utilities|FlowControl|Delay 0.2)
                              (Rendering|SetVisibility (Variables|Default|GetTextButton4) false false)
                              (Rendering|SetVisibility (Variables|Default|GetTextButton4Red) true false))
                            (:then_2
                              (goto _label_4)))))))))))
          (:then_1
            (if (== (Variables|Default|GetPasswordIndex) 1)
              (if (== (Variables|Default|GetNumPressed) (Utilities|Array|Get(acopy) (Variables|Default|GetPassword) 1))
                (goto _label)
                (else
                  (goto _label_3)))))
          (:then_2
            (if (== (Variables|Default|GetPasswordIndex) 2)
              (if (== (Variables|Default|GetNumPressed) (Utilities|Array|Get(acopy) (Variables|Default|GetPassword) 2))
                (goto _label)
                (else
                  (goto _label_3)))))
          (:then_3
            (if (== (Variables|Default|GetPasswordIndex) 3)
              (if (== (Variables|Default|GetNumPressed) (Utilities|Array|Get(acopy) (Variables|Default|GetPassword) 3))
                (Utilities|FlowControl|Sequence
                  (:then_0
                    (goto _label))
                  (:then_1
                    (Utilities|FlowControl|Gate true
                      (:Exit
                        (Utilities|FlowControl|Delay 0.2)
                        (Rendering|SetVisibility (Variables|Default|GetBlueScreen) false false)
                        (Rendering|SetVisibility (Variables|Default|GetGreenScreen) true false)
                        (Widget|RemovefromParent (stale OnComponentBeginOverlap(Trigger) _returnvalue_2))
                        (Variables|Default|SetDoorOpened true)
                        (Audio|PlaySound2D "/Engine/VREditor/Sounds/UI/Click_on_Button_Cue.Click_on_Button_Cue" 2.0 1.0 0.0 0 0)
                        (Audio|PlaySoundatLocation "/Game/Maps/AMalginov/BluePrints/Sound_Lock-Click.Sound_Lock-Click" _returnvalue_3 "0, 0, 0" 0.2 1.0 0.0 0 0 0 0)
                        (Utilities|FlowControl|Sequence
                          (:then_0
                            (Utilities|FlowControl|Delay 1.0)
                            (bind _newtrack_0_5 (Timeline|Door%20Rotation Play)
                              (:Update
                                (Transformation|SetRelativeRotation (Variables|Default|GetDoor) (Math|Rotator|MakeRotator 0.0 0.0 _newtrack_0_5) false false))))
                          (:then_1
                            (Utilities|FlowControl|Delay 0.6)
                            (Audio|PlaySoundatLocation "/Game/Maps/AMalginov/BluePrints/Sound_Opening-of-a-big-rusty-metal-door.Sound_Opening-of-a-big-rusty-metal-door" _returnvalue_3 "0, 0, 0" 0.5 1.0 0.0 0 0 0 0)))
                        (Utilities|FlowControl|Delay 4.0)
                        (goto _label_5)))))
                (else
                  (goto _label_3))))))))))

(fn ConstructionScript)