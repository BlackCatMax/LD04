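; BP_EndGame is a trigger actor that runs the game's ending sequence when the player character overlaps it.
; It disables player input, clears widgets, blends the view to itself, plays a sound and animates post-process exposure through a timeline.
; It then steps WB_EndGame through timed slides.
; On the fourth slide it opens a gate so pressing F shows the fifth and loads L_MainMap.
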(event OnComponentBeginOverlap(Trigger)
  (params (OverlappedComponent :type Primitive%20Component%20Object%20Reference) (OtherActor :type Actor%20Object%20Reference) (OtherComp :type Primitive%20Component%20Object%20Reference) (OtherBodyIndex :type Integer) (bFromSweep :type Boolean) (SweepResult :type Hit%20Result%20Structure%20%28by%20ref%29))
  (if (== OtherActor (Game|GetPlayerCharacter 0))
    (Utilities|FlowControl|Sequence
      (:then_0
        (Utilities|FlowControl|Delay 0.4)
        (Rendering|SetVisibility (Variables|Default|GetPostProcess) true false)
        (bind _exposure_compensation (Timeline|Changing%20PostProcess Play)
          (:Update
            (Variables|/Script/Engine.PostProcessComponent|SetSettings (Variables|Default|GetPostProcess) (Utilities|Struct|MakePostProcessSettings _exposure_compensation)))
          (:Finished
            (bind _returnvalue (UserInterface|CreateWidget "/Game/Maps/AMalginov/Widgets/WB_EndGame.WB_EndGame_C" (Game|GetPlayerController 0)))
            (UserInterface|Viewport|AddtoViewport _returnvalue 0)
            (Utilities|FlowControl|Delay 3.0)
            (Variables|/Game/Maps/AMalginov/Widgets/WB_EndGame.WB_EndGame_C|SetTheEndVisibility _returnvalue false)
            (Variables|/Game/Maps/AMalginov/Widgets/WB_EndGame.WB_EndGame_C|SetSlide_1Visibility _returnvalue true)
            (Utilities|FlowControl|Delay 5.0)
            (Variables|/Game/Maps/AMalginov/Widgets/WB_EndGame.WB_EndGame_C|SetSlide_1Visibility _returnvalue false)
            (Variables|/Game/Maps/AMalginov/Widgets/WB_EndGame.WB_EndGame_C|SetSlide_2Visibility _returnvalue true)
            (Utilities|FlowControl|Delay 5.0)
            (Variables|/Game/Maps/AMalginov/Widgets/WB_EndGame.WB_EndGame_C|SetSlide_2Visibility _returnvalue false)
            (Variables|/Game/Maps/AMalginov/Widgets/WB_EndGame.WB_EndGame_C|SetSlide_3Visibility _returnvalue true)
            (Utilities|FlowControl|Delay 5.0)
            (Variables|/Game/Maps/AMalginov/Widgets/WB_EndGame.WB_EndGame_C|SetSlide_3Visibility _returnvalue false)
            (Variables|/Game/Maps/AMalginov/Widgets/WB_EndGame.WB_EndGame_C|SetSlide_4Visibility _returnvalue true)
            (Input|EnableInput (Game|GetPlayerController 0))
            (Utilities|FlowControl|Gate true) ; enters at Open
          )))
      (:then_1
        (Game|Player|SetViewTargetwithBlend (Game|GetPlayerController 0) self 2.0 "VTBlend_Linear" 0.0 false))
      (:then_2
        (Input|DisableInput (Game|GetPlayerCharacter 0) (Game|GetPlayerController 0))
        (Viewport|RemoveAllWidgets)
        (Utilities|FlowControl|Delay 1.0)
        (Audio|PlaySound2D "/Game/Maps/AMalginov/Sounds/Sound_You-Are-My-Rainbow-Unicorn-Heads_Cue.Sound_You-Are-My-Rainbow-Unicorn-Heads_Cue" 1.0 1.0 0.0 0 0)))))

(event Input|KeyboardEvents|F
  (params (Key :type Key%20Structure :default "None"))
  (:Pressed
    (Utilities|FlowControl|Gate true
      (:Exit
        (Variables|/Game/Maps/AMalginov/Widgets/WB_EndGame.WB_EndGame_C|SetSlide_4Visibility (stale OnComponentBeginOverlap(Trigger) _returnvalue) false)
        (Variables|/Game/Maps/AMalginov/Widgets/WB_EndGame.WB_EndGame_C|SetSlide_5Visibility (stale OnComponentBeginOverlap(Trigger) _returnvalue) true)
        (Game|OpenLevel(byName) "L_MainMap")))))

(fn ConstructionScript)