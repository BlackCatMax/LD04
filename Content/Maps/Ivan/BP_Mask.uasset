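; BP_Mask is an interactable prop that the player triggers with E while standing in its Box volume.
; Overlap by the ALS_AnimMan character enables input, shows the TextRender1 prompt and opens a Gate; leaving disables input, hides both texts and closes it.
; Pressing E through the Gate destroys the prompt and plays a Timeline that yaws SuperGridBox19 at a fixed relative location while showing TextRender.
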(event OnComponentBeginOverlap(Box)
  (params (OverlappedComponent :type Primitive%20Component%20Object%20Reference) (OtherActor :type Actor%20Object%20Reference) (OtherComp :type Primitive%20Component%20Object%20Reference) (OtherBodyIndex :type Integer) (bFromSweep :type Boolean) (SweepResult :type Hit%20Result%20Structure%20%28by%20ref%29))
  (Utilities|Casting|CastToALS_AnimMan_CharacterBP OtherActor)
  (Input|EnableInput (Game|GetPlayerController 0))
  (Rendering|SetVisibility (Variables|Default|GetTextRender1) true false)
  (Utilities|FlowControl|Gate true) ; enters at Open
)

(event OnComponentEndOverlap(Box)
  (params (OverlappedComponent :type Primitive%20Component%20Object%20Reference) (OtherActor :type Actor%20Object%20Reference) (OtherComp :type Primitive%20Component%20Object%20Reference) (OtherBodyIndex :type Integer))
  (Utilities|Casting|CastToALS_AnimMan_CharacterBP OtherActor)
  (Input|DisableInput (Game|GetPlayerController 0))
  (Rendering|SetVisibility (Variables|Default|GetTextRender1) false false)
  (Utilities|FlowControl|Gate true) ; enters at Close
)

(event Input|KeyboardEvents|E
  (params (Key :type Key%20Structure :default "None"))
  (:Pressed
    (Utilities|FlowControl|Gate true
      (:Exit
        (Components|DestroyComponent (Variables|Default|GetTextRender1))
        (bind _newtrack_0 (Timeline|Timeline Play)
          (:Update
            (Transformation|SetRelativeLocationAndRotation (Variables|Default|GetSuperGrid_Box19) (Math|Vector|MakeVector -41.013335 -71.251739 -1.6e-05) (Math|Rotator|MakeRotator 0.0 0.0 _newtrack_0) false false)
            (Rendering|SetVisibility (Variables|Default|GetTextRender) true false)))))))

(fn ConstructionScript)