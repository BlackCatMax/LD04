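; Interactable wood block actor that swaps one SuperGridBox for another when the player presses E nearby.
; A Box overlap by the ALS_AnimMan character enables input, shows a TextRender prompt and opens a Gate; leaving reverses all three.
; Pressing E through the open Gate destroys the prompt, hides SuperGridBox, then reveals SuperGridBox1 and turns on its collision.
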(event OnComponentBeginOverlap(Box)
  (params (OverlappedComponent :type Primitive%20Component%20Object%20Reference) (OtherActor :type Actor%20Object%20Reference) (OtherComp :type Primitive%20Component%20Object%20Reference) (OtherBodyIndex :type Integer) (bFromSweep :type Boolean) (SweepResult :type Hit%20Result%20Structure%20%28by%20ref%29))
  (bind _supergrid_box1 (Variables|Default|GetSuperGrid_Box1))
  (Utilities|Casting|CastToALS_AnimMan_CharacterBP OtherActor)
  (Input|EnableInput (Game|GetPlayerController 0))
  (Rendering|SetVisibility (Variables|Default|GetTextRender) true false)
  (Utilities|FlowControl|Gate true) ; enters at Open
)

(event OnComponentEndOverlap(Box)
  (params (OverlappedComponent :type Primitive%20Component%20Object%20Reference) (OtherActor :type Actor%20Object%20Reference) (OtherComp :type Primitive%20Component%20Object%20Reference) (OtherBodyIndex :type Integer))
  (bind _supergrid_box1 (Variables|Default|GetSuperGrid_Box1))
  (Utilities|Casting|CastToALS_AnimMan_CharacterBP OtherActor)
  (Input|DisableInput (Game|GetPlayerController 0))
  (Rendering|SetVisibility (Variables|Default|GetTextRender) false false)
  (Utilities|FlowControl|Gate true) ; enters at Close
)

(event Input|KeyboardEvents|E
  (params (Key :type Key%20Structure :default "None"))
  (bind _supergrid_box1 (Variables|Default|GetSuperGrid_Box1))
  (:Pressed
    (Utilities|FlowControl|Gate true
      (:Exit
        (Components|DestroyComponent (Variables|Default|GetTextRender))
        (Rendering|SetVisibility (Variables|Default|GetSuperGrid_Box) false false)
        (Rendering|SetVisibility _supergrid_box1 true false)
        (Collision|SetCollisionEnabled _supergrid_box1 "QueryAndPhysics")))))

(fn ConstructionScript)