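; BP_Mount is an interactable pickup that grants the player character its Mount state.
; Box overlap with an ALS_AnimMan_CharacterBP stores that character, enables player input, shows a text prompt and opens a gate; leaving reverses the input, text and gate.
; Pressing E through the open gate sets the character's Mount flag to true, prints it, waits briefly and destroys the actor.
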(event OnComponentBeginOverlap(Box)
  (params (OverlappedComponent :type Primitive%20Component%20Object%20Reference) (OtherActor :type Actor%20Object%20Reference) (OtherComp :type Primitive%20Component%20Object%20Reference) (OtherBodyIndex :type Integer) (bFromSweep :type Boolean) (SweepResult :type Hit%20Result%20Structure%20%28by%20ref%29))
  (bind _asals_anim_man_character_bp (Utilities|Casting|CastToALS_AnimMan_CharacterBP OtherActor))
  (Variables|Default|SetAs%20ALS%20Anim%20Man%20Character%20BP _asals_anim_man_character_bp)
  (Input|EnableInput (Game|GetPlayerController 0))
  (Rendering|SetVisibility (Variables|Default|GetTextRender) true false)
  (Utilities|FlowControl|Gate true) ; enters at Open
)

(event OnComponentEndOverlap(Box)
  (params (OverlappedComponent :type Primitive%20Component%20Object%20Reference) (OtherActor :type Actor%20Object%20Reference) (OtherComp :type Primitive%20Component%20Object%20Reference) (OtherBodyIndex :type Integer))
  (Utilities|Casting|CastToALS_AnimMan_CharacterBP OtherActor)
  (Input|DisableInput (Game|GetPlayerController 0))
  (Rendering|SetVisibility (Variables|Default|GetTextRender) false false)
  (Utilities|FlowControl|Gate true) ; enters at Close
)

(event Input|KeyboardEvents|E
  (params (Key :type Key%20Structure))
  (:Pressed
    (Utilities|FlowControl|Gate true
      (:Exit
        (bind _output_get (Variables|/Game/AdvancedLocomotionV4/Blueprints/CharacterLogic/ALS_AnimMan_CharacterBP.ALS_AnimMan_CharacterBP_C|SetMount (Variables|Default|GetAs%20ALS%20Anim%20Man%20Character%20BP) true))
        (Development|PrintString (Utilities|String|ToString(Boolean) _output_get) true true "(R=0.000000,G=1.000000,B=0.045587,A=1.000000)")
        (Utilities|FlowControl|Delay 0.2)
        (Actor|DestroyActor)))))

(fn ConstructionScript)