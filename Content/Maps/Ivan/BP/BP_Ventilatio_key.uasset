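; Interactive ventilation grille that rotates when the player presses E inside its trigger box, provided the character's Mount flag is true.
; Box overlap toggles input, the prompt text and a gate on the key action.
; The action destroys the prompt, reveals a second text and plays a timeline driving Grid2's roll.
; Mount is read from the cast in the end-overlap event, not begin-overlap.
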(event OnComponentBeginOverlap(Box)
  (params (OverlappedComponent :type Primitive%20Component%20Object%20Reference) (OtherActor :type Actor%20Object%20Reference) (OtherComp :type Primitive%20Component%20Object%20Reference) (OtherBodyIndex :type Integer) (bFromSweep :type Boolean) (SweepResult :type Hit%20Result%20Structure%20%28by%20ref%29))
  (Utilities|Casting|CastToALS_AnimMan_CharacterBP OtherActor)
  (Input|EnableInput (Game|GetPlayerController 0))
  (Rendering|SetVisibility (Variables|Default|GetTextRender) true false)
  (Utilities|FlowControl|Gate true) ; enters at Open
)

(event OnComponentEndOverlap(Box)
  (params (OverlappedComponent :type Primitive%20Component%20Object%20Reference) (OtherActor :type Actor%20Object%20Reference) (OtherComp :type Primitive%20Component%20Object%20Reference) (OtherBodyIndex :type Integer))
  (bind _asals_anim_man_character_bp (Utilities|Casting|CastToALS_AnimMan_CharacterBP OtherActor))
  (Input|DisableInput (Game|GetPlayerController 0))
  (Rendering|SetVisibility (Variables|Default|GetTextRender) false false)
  (Utilities|FlowControl|Gate true) ; enters at Close
)

(event Input|KeyboardEvents|E
  (params (Key :type Key%20Structure))
  (:Pressed
    (if (Variables|/Game/AdvancedLocomotionV4/Blueprints/CharacterLogic/ALS_AnimMan_CharacterBP.ALS_AnimMan_CharacterBP_C|GetMount (stale OnComponentEndOverlap(Box) _asals_anim_man_character_bp))
      (Utilities|FlowControl|Gate true
        (:Exit
          (Rendering|SetVisibility (Variables|Default|GetTextRender1) true false)
          (Components|DestroyComponent (Variables|Default|GetTextRender))
          (bind _newtrack_0 (Timeline|Timeline Play)
            (:Update
              (Transformation|SetRelativeLocationAndRotation (Variables|Default|GetGrid_2) (Math|Vector|MakeVector 0.0 0.0 0.0) (Math|Rotator|MakeRotator _newtrack_0 0.0 0.0) false false))))))))

(fn ConstructionScript)