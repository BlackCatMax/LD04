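; Elevator activator that lets the ALS player character press E inside a trigger box to start a one-shot scripted elevator sequence.
; Overlap toggles input, a text prompt and a Gate; pressing E removes the prompt and runs chained, delayed timelines that move meshes with hard-coded relative positions and play sounds.
; A second trigger separately slides the same pair of door-like boxes after a delay, plays the metal door sound and destroys itself.
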(event OnComponentBeginOverlap(Box)
  (params (OverlappedComponent :type Primitive%20Component%20Object%20Reference) (OtherActor :type Actor%20Object%20Reference) (OtherComp :type Primitive%20Component%20Object%20Reference) (OtherBodyIndex :type Integer) (bFromSweep :type Boolean) (SweepResult :type Hit%20Result%20Structure%20%28by%20ref%29))
  (bind _sm_merged_staticmeshactor_500 (Variables|Default|GetSM_MERGED_StaticMeshActor_500))
  (Utilities|Casting|CastToALS_AnimMan_CharacterBP OtherActor)
  (Input|EnableInput (Game|GetPlayerController 0))
  (Rendering|SetVisibility (Variables|Default|GetTextRender) true false)
  (Utilities|FlowControl|Gate true) ; enters at Open
)

(event OnComponentEndOverlap(Box)
  (params (OverlappedComponent :type Primitive%20Component%20Object%20Reference) (OtherActor :type Actor%20Object%20Reference) (OtherComp :type Primitive%20Component%20Object%20Reference) (OtherBodyIndex :type Integer))
  (bind _sm_merged_staticmeshactor_500 (Variables|Default|GetSM_MERGED_StaticMeshActor_500))
  (Utilities|Casting|CastToALS_AnimMan_CharacterBP OtherActor)
  (Input|DisableInput (Game|GetPlayerController 0))
  (Rendering|SetVisibility (Variables|Default|GetTextRender) false false)
  (Utilities|FlowControl|Gate true) ; enters at Close
)

(event OnComponentBeginOverlap(Box1)
  (params (OverlappedComponent :type Primitive%20Component%20Object%20Reference) (OtherActor :type Actor%20Object%20Reference) (OtherComp :type Primitive%20Component%20Object%20Reference) (OtherBodyIndex :type Integer) (bFromSweep :type Boolean) (SweepResult :type Hit%20Result%20Structure%20%28by%20ref%29))
  (Utilities|Casting|CastToALS_AnimMan_CharacterBP OtherActor)
  (Utilities|FlowControl|Delay 1.0)
  (bind _newtrack_0 (Timeline|Timeline_5 Play)
    (:Update
      (Transformation|SetRelativeLocationAndRotation (Variables|Default|GetSuperGrid_Box10) (Math|Vector|MakeVector -269.488539 _newtrack_0 -1305.393796) "0, 0, 0" false false)
      (bind _newtrack_0_2 (Timeline|Timeline_6 Play)
        (:Update
          (Transformation|SetRelativeLocationAndRotation (Variables|Default|GetSuperGrid_Box9) (Math|Vector|MakeVector -269.488539 _newtrack_0_2 -1305.393796) "0, 0, 0" false false)
          (Utilities|FlowControl|DoOnce false
            (:Completed
              (Audio|PlaySound2D "/Game/Maps/Ivan/Sounds/Soubd_Metall_door_Elevator.Soubd_Metall_door_Elevator" 1.0 1.0 0.0 0 0)
              (Components|DestroyComponent (Variables|Default|GetBox1)))))))))

(event Input|KeyboardEvents|E
  (params (Key :type Key%20Structure))
  (bind _sm_merged_staticmeshactor_500 (Variables|Default|GetSM_MERGED_StaticMeshActor_500))
  (:Pressed
    (Utilities|FlowControl|Gate true
      (:Exit
        (Components|DestroyComponent (Variables|Default|GetTextRender))
        (bind _newtrack_0 (Timeline|Timeline_4 Play)
          (:Update
            (Transformation|SetRelativeLocationAndRotation (Variables|Default|GetSuperGrid_Box2) (Math|Vector|MakeVector _newtrack_0 -10.487205 157.192473) "0, 0, 0" false false)
            (Components|DestroyComponent (Variables|Default|GetSuperGrid_Box7))
            (bind _newtrack_0_2 (Timeline|Timeline Play)
              (:Update
                (Rendering|SetVisibility _sm_merged_staticmeshactor_500 true false)
                (Transformation|SetRelativeLocationAndRotation _sm_merged_staticmeshactor_500 (Math|Vector|MakeVector -234.545263 -44.377099 _newtrack_0_2) "0, 0, 0" false false)
                (Utilities|FlowControl|Delay 2.0)
                (Utilities|FlowControl|DoOnce false
                  (:Completed
                    (Audio|PlaySound2D "/Game/Maps/Ivan/Sounds/bb1f99b2f2850e4.bb1f99b2f2850e4" 1.0 1.0 0.0 0 0)
                    (Utilities|FlowControl|Delay 3.0)
                    (bind _newtrack_1 (Timeline|Timeline_0 Play)
                      (:Update
                        (Transformation|SetRelativeLocationAndRotation (Variables|Default|GetSuperGrid_Box4) (Math|Vector|MakeVector -232.535994 -122.918469 _newtrack_1) "0, 0, 0" false false)
                        (bind _newtrack_0_3 (Timeline|Timeline_1 Play)
                          (:Update
                            (Transformation|SetRelativeLocationAndRotation (Variables|Default|GetSuperGrid_Box5) (Math|Vector|MakeVector -232.535994 -122.918469 _newtrack_0_3) "0, 0, 0" false false)
                            (Utilities|FlowControl|Delay 6.5)
                            (bind _newtrack_0_4 (Timeline|Timeline_2 Play)
                              (:Update
                                (Transformation|SetRelativeLocationAndRotation (Variables|Default|GetSuperGrid_Box10) (Math|Vector|MakeVector -269.488539 _newtrack_0_4 -1305.393796) "0, 0, 0" false false)
                                (bind _newtrack_0_5 (Timeline|Timeline_3 Play)
                                  (:Update
                                    (Transformation|SetRelativeLocationAndRotation (Variables|Default|GetSuperGrid_Box9) (Math|Vector|MakeVector -269.488539 _newtrack_0_5 -1305.393796) "0, 0, 0" false false)
                                    (Utilities|FlowControl|DoOnce false
                                      (:Completed
                                        (Audio|PlaySound2D "/Game/Maps/Ivan/Sounds/Soubd_Metall_door_Elevator.Soubd_Metall_door_Elevator" 1.0 1.0 0.0 0 0)))))))))))))))))))))

(fn ConstructionScript)