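; Keycard door that slides open when the player presses E while carrying the second keycard (KeyCard2L).
; A box overlap with the ALS character enables input, shows prompt texts and opens a Gate that lets the key press through.
; With the card, it hides one pair of cylinder meshes, plays a sound and slides the door along X via timeline.
; Without it, another pair hides for two seconds with a different sound, then the gate closes.
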(event OnComponentBeginOverlap(Box)
  (params (OverlappedComponent :type Primitive%20Component%20Object%20Reference) (OtherActor :type Actor%20Object%20Reference) (OtherComp :type Primitive%20Component%20Object%20Reference) (OtherBodyIndex :type Integer) (bFromSweep :type Boolean) (SweepResult :type Hit%20Result%20Structure%20%28by%20ref%29))
  (bind _supergrid_cylinderfull1 (Variables|Default|GetSuperGrid_CylinderFull1))
  (bind _asals_anim_man_character_bp (Utilities|Casting|CastToALS_AnimMan_CharacterBP OtherActor))
  (Input|EnableInput (Game|GetPlayerController 0))
  (Rendering|SetVisibility (Variables|Default|GetTextRender) true false)
  (Utilities|FlowControl|Gate true) ; enters at Open
)

(event OnComponentEndOverlap(Box)
  (params (OverlappedComponent :type Primitive%20Component%20Object%20Reference) (OtherActor :type Actor%20Object%20Reference) (OtherComp :type Primitive%20Component%20Object%20Reference) (OtherBodyIndex :type Integer))
  (bind _supergrid_cylinderfull1 (Variables|Default|GetSuperGrid_CylinderFull1))
  (Utilities|Casting|CastToALS_AnimMan_CharacterBP OtherActor)
  (Input|DisableInput (Game|GetPlayerController 0))
  (Rendering|SetVisibility (Variables|Default|GetTextRender) false false)
  (Utilities|FlowControl|Gate true) ; enters at Close
)

(event Input|KeyboardEvents|E
  (params (Key :type Key%20Structure :default "None"))
  (bind _supergrid_cylinderfull1 (Variables|Default|GetSuperGrid_CylinderFull1))
  (:Pressed
    (Utilities|FlowControl|Gate true :!label _label
      (:Exit
        (if (Variables|/Game/AdvancedLocomotionV4/Blueprints/CharacterLogic/ALS_AnimMan_CharacterBP.ALS_AnimMan_CharacterBP_C|GetKey_card_2L (stale OnComponentBeginOverlap(Box) _asals_anim_man_character_bp))
          (Rendering|SetVisibility (Variables|Default|GetSuperGrid_CylinderFull) false false)
          (Audio|PlaySound2D "/Game/Maps/Ivan/Sounds/KeycardUse1.KeycardUse1" 1.0 1.0 0.0 0 0)
          (bind _newtrack_0 (Timeline|Timeline Play)
            (:Update
              (Transformation|SetRelativeLocationAndRotation (Variables|Default|GetSuperGrid_Box) (Math|Vector|MakeVector _newtrack_0 0.0 0.0) "0, 0, 0" false false)))
          (else
            (Rendering|SetVisibility _supergrid_cylinderfull1 false false)
            (Audio|PlaySound2D "/Game/Maps/Ivan/Sounds/KeycardUse2.KeycardUse2" 1.0 1.0 0.0 0 0)
            (Utilities|FlowControl|Delay 2.0)
            (Rendering|SetVisibility _supergrid_cylinderfull1 true false)
            (goto _label Close)))))))

(fn ConstructionScript)