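; Two-stage press-E activator that lets the player rotate and move grid-box props, apparently a door and a switch-driven mechanism.
; Trigger boxes show text prompts, enable input and open Gates while the ALS character overlaps.
; The first press plays a yaw timeline, removes its trigger and repositions the second.
; The second chains a roll timeline into a height timeline, swaps spotlights and activates a door sound once.
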(event OnComponentBeginOverlap(Box)
  (params (OverlappedComponent :type Primitive%20Component%20Object%20Reference) (OtherActor :type Actor%20Object%20Reference) (OtherComp :type Primitive%20Component%20Object%20Reference) (OtherBodyIndex :type Integer) (bFromSweep :type Boolean) (SweepResult :type Hit%20Result%20Structure%20%28by%20ref%29))
  (Utilities|Casting|CastToALS_AnimMan_CharacterBP OtherActor)
  (Input|EnableInput (Game|GetPlayerController 0))
  (Rendering|SetVisibility (Variables|Default|GetTextRender) true false)
  (Utilities|FlowControl|Gate true) ; enters at Open
)

(event OnComponentEndOverlap(Box)
  (params (OverlappedComponent :type Primitive%20Component%20Object%20Reference) (OtherActor :type Actor%20Object%20Reference) (OtherComp :type Primitive%20Component%20Object%20Reference) (OtherBodyIndex :type Integer))
  (Utilities|Casting|CastToALS_AnimMan_CharacterBP OtherActor)
  (Input|DisableInput (Game|GetPlayerController 0))
  (Rendering|SetVisibility (Variables|Default|GetTextRender) false false)
  (Utilities|FlowControl|Gate true) ; enters at Close
)

(event OnComponentBeginOverlap(Box1)
  (params (OverlappedComponent :type Primitive%20Component%20Object%20Reference) (OtherActor :type Actor%20Object%20Reference) (OtherComp :type Primitive%20Component%20Object%20Reference) (OtherBodyIndex :type Integer) (bFromSweep :type Boolean) (SweepResult :type Hit%20Result%20Structure%20%28by%20ref%29))
  (Utilities|Casting|CastToALS_AnimMan_CharacterBP OtherActor)
  (Input|EnableInput (Game|GetPlayerController 0))
  (Rendering|SetVisibility (Variables|Default|GetTextRender1) true false)
  (Utilities|FlowControl|Gate true) ; enters at Open
)

(event OnComponentEndOverlap(Box1)
  (params (OverlappedComponent :type Primitive%20Component%20Object%20Reference) (OtherActor :type Actor%20Object%20Reference) (OtherComp :type Primitive%20Component%20Object%20Reference) (OtherBodyIndex :type Integer))
  (Utilities|Casting|CastToALS_AnimMan_CharacterBP OtherActor)
  (Input|DisableInput (Game|GetPlayerController 0))
  (Rendering|SetVisibility (Variables|Default|GetTextRender1) false false)
  (Utilities|FlowControl|Gate true) ; enters at Close
)

(event Input|KeyboardEvents|E
  (params (Key :type Key%20Structure))
  (:Pressed
    (Utilities|FlowControl|Gate true
      (:Exit
        (bind _newtrack_0 (Timeline|Timeline_0 Play)
          (:Update
            (Transformation|SetRelativeRotation (Variables|Default|GetSuperGrid_Box7) (Math|Rotator|MakeRotator _newtrack_0 0.0 0.0) false false)
            (Components|DestroyComponent (Variables|Default|GetTextRender1))
            (bind _newtrack_0_2 (Timeline|Timeline_1 Play)
              (:Update
                (Transformation|SetRelativeLocationAndRotation (Variables|Default|GetSuperGrid_Box10) (Math|Vector|MakeVector -5988.440684 3059.283979 _newtrack_0_2) "0.000000,40.000000,0.000000" false false)
                (Components|DestroyComponent (Variables|Default|GetSpotLight))
                (Rendering|SetVisibility (Variables|Default|GetSpotLight1) true false)
                (Utilities|FlowControl|DoOnce false
                  (:Completed
                    (Components|Activation|Activate (Variables|Default|GetSound_Door1) false)))))))))))

(event Input|KeyboardEvents|E
  (params (Key :type Key%20Structure))
  (:Pressed
    (Utilities|FlowControl|Gate true
      (:Exit
        (Components|DestroyComponent (Variables|Default|GetTextRender))
        (if (Variables|Default|GetDoorOpen)
          (bind _newtrack_0 (Timeline|Timeline Play)
            (:Update
              (Transformation|SetRelativeRotation (Variables|Default|GetSuperGrid_Box5) (Math|Rotator|MakeRotator 0.0 0.0 _newtrack_0) false false)
              (Variables|Default|SetDoorOpen (not (> _newtrack_0 0.0)))
              (Components|DestroyComponent (Variables|Default|GetBox))
              (Transformation|SetRelativeLocationAndRotation (Variables|Default|GetBox1) (Math|Vector|MakeVector 0.0 0.0 -193.0) "0, 0, 0" false false)))
          (else
            (Timeline|Timeline ReverseFromEnd)))))))

(fn ConstructionScript)