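; Interactive glass door that the player opens once by pressing E while standing next to it.
; A trigger box detects the ALS character, toggling player input, a prompt TextRender and a Gate that only passes E while inside.
; On use, the prompt is destroyed and a Timeline drives the yaw of the SuperGridBox door mesh around a fixed relative location.
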(event OnComponentBeginOverlap(Box)
  (params (OverlappedComponent :type Primitive%20Component%20Object%20Reference) (OtherActor :type Actor%20Object%20Reference) (OtherComp :type Primitive%20Component%20Object%20Reference) (OtherBodyIndex :type Integer) (bFromSweep :type Boolean) (SweepResult :type Hit%20Result%20Structure%20%28by%20ref%29))
  (Utilities|Casting|CastToALS_AnimMan_CharacterBP OtherActor)
  (Input|EnableInput (Game|GetPlayerController 0))
  (Rendering|SetVisibility (Variables|Default|GetTextRender) true false)
  (Utilities|FlowControl|Gate true) ; enters at Open
)

(event OnComponentEndOverlap(Box)
  (params (OverlappedComponent :type Primitive%20Component%20Object%20Reference) (OtherActor :type Actor%20Object%20Reference) (OtherComp :type Primitive%20Component%20Object%20Reference) (OtherBodyIndex :type Integer))
  (Utilities|Casting|CastToALS_AnimMan_CharacterBP OtherActor)
  (Input|DisableInput (Game|GetPlayerController 0))
  (Rendering|SetVisibility (Variables|Default|GetTextRender) false false)
  (Utilities|FlowControl|Gate true) ; enters at Close
)

(event Input|KeyboardEvents|E
  (params (Key :type Key%20Structure))
  (:Pressed
    (Utilities|FlowControl|Gate true
      (:Exit
        (Components|DestroyComponent (Variables|Default|GetTextRender))
        (bind _newtrack_0 (Timeline|Timeline Play)
          (:Update
            (Transformation|SetRelativeLocationAndRotation (Variables|Default|GetSuperGrid_Box) (Math|Vector|MakeVector -17.680144 -72.120019 29.489131) (Math|Rotator|MakeRotator 0.0 0.0 _newtrack_0) false false)))))))

(fn ConstructionScript)