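; Elevator activator that lets the ALS player character press E inside a trigger box to set elevator meshes moving.
; Box overlap toggles input, a text prompt and a Gate on the key press.
; Pressing E destroys the prompt and plays a timeline that reveals and moves a merged mesh along Z.
; Its update also starts a three-second Delay, then two chained timelines move two SuperGridBox meshes along Z.
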(event OnComponentBeginOverlap(Box)
  (params (OverlappedComponent :type Primitive%20Component%20Object%20Reference) (OtherActor :type Actor%20Object%20Reference) (OtherComp :type Primitive%20Component%20Object%20Reference) (OtherBodyIndex :type Integer) (bFromSweep :type Boolean) (SweepResult :type Hit%20Result%20Structure%20%28by%20ref%29))
  (bind _sm_merged_staticmeshactor_500 (Variables|Default|GetSM_MERGED_StaticMeshActor_500))
  (Utilities|Casting|CastToALS_AnimMan_CharacterBP OtherActor)
  (Input|EnableInput (Game|GetPlayerController 0))
  (Rendering|SetVisibility (Variables|Default|GetTextRender) true false)
  (Utilities|FlowControl|Gate true) ; enters at Open
)

(event OnComponentEndOverlap(Box)
  (params (OverlappedComponent :type Primitive%20Component%20Object%20Reference) (OtherActor :type Actor%20Object%20Reference) (OtherComp :type Primitive%20Component%20Object%20Reference) (OtherBodyIndex :type Integer))
  (bind _sm_merged_staticmeshactor_500 (Variables|Default|GetSM_MERGED_StaticMeshActor_500))
  (Utilities|Casting|CastToALS_AnimMan_CharacterBP OtherActor)
  (Input|DisableInput (Game|GetPlayerController 0))
  (Rendering|SetVisibility (Variables|Default|GetTextRender) false false)
  (Utilities|FlowControl|Gate true) ; enters at Close
)

(event Input|KeyboardEvents|E
  (params (Key :type Key%20Structure :default "None"))
  (bind _sm_merged_staticmeshactor_500 (Variables|Default|GetSM_MERGED_StaticMeshActor_500))
  (:Pressed
    (Utilities|FlowControl|Gate true
      (:Exit
        (Components|DestroyComponent (Variables|Default|GetTextRender))
        (bind _newtrack_0 (Timeline|Timeline Play)
          (:Update
            (Rendering|SetVisibility _sm_merged_staticmeshactor_500 true false)
            (Transformation|SetRelativeLocationAndRotation _sm_merged_staticmeshactor_500 (Math|Vector|MakeVector -234.545263 -44.377099 _newtrack_0) "0.000000,0.000000,0.000000" false false)
            (Utilities|FlowControl|Delay 3.0)
            (bind _newtrack_1 (Timeline|Timeline_0 Play)
              (:Update
                (Transformation|SetRelativeLocationAndRotation (Variables|Default|GetSuperGrid_Box4) (Math|Vector|MakeVector -232.535994 -122.918469 _newtrack_1) "0.000000,0.000000,0.000000" false false)
                (bind _newtrack_0_2 (Timeline|Timeline_1 Play)
                  (:Update
                    (Transformation|SetRelativeLocationAndRotation (Variables|Default|GetSuperGrid_Box5) (Math|Vector|MakeVector -232.535994 -122.918469 _newtrack_0_2) "0, 0, 0" false false)))))))))))

(fn ConstructionScript)