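; BP_Button_3 is a wall or world button that opens a linked Door when the player presses Interaction nearby.
; Box overlaps with the ALS character toggle a Gate on the input.
; One graph slides the button in and back with timelines, messaging the Door through an interface on each update.
; A second graph requires a working generator, squashes the button's scale, then calls OpenDoor, otherwise printing a repair notice.
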(event OnComponentBeginOverlap(Box)
  (params (OverlappedComponent :type Primitive%20Component%20Object%20Reference) (OtherActor :type Actor%20Object%20Reference) (OtherComp :type Primitive%20Component%20Object%20Reference) (OtherBodyIndex :type Integer) (bFromSweep :type Boolean) (SweepResult :type Hit%20Result%20Structure%20%28by%20ref%29))
  (Utilities|Casting|CastToALS_AnimMan_CharacterBP OtherActor)
  (Utilities|FlowControl|Gate true) ; enters at Open
)

(event OnComponentEndOverlap(Box)
  (params (OverlappedComponent :type Primitive%20Component%20Object%20Reference) (OtherActor :type Actor%20Object%20Reference) (OtherComp :type Primitive%20Component%20Object%20Reference) (OtherBodyIndex :type Integer))
  (Utilities|Casting|CastToALS_AnimMan_CharacterBP OtherActor)
  (Utilities|FlowControl|Gate true) ; enters at Close
)

(event EventBeginPlay
  (bind _button (Variables|Default|GetButton))
  (bind _returnvalue (Transformation|GetRelativeTransform _button))
  ;[1 1 1] set button start location
  (Variables|Default|SetButton%20out (Math|Transform|MakeTransform (.location _returnvalue) (.rotation _returnvalue) (.scale _returnvalue)))
  (Variables|Default|SetButton%20in (Math|Transform|MakeTransform (- (.location _returnvalue) "0.000000,-50.000000,0.000000") (.rotation _returnvalue) (.scale _returnvalue)))
  (Input|EnableInput (Game|GetPlayerController 0)))

(event EventTick
  (params (DeltaSeconds :type Float%20%28single-precision%29))
  (bind _button (Variables|Default|GetButton))
  (bind _relativelocation (Variables|/Script/Engine.SceneComponent|GetRelativeLocation _button))
  ;[1 1 1] sound
  (if (not (<= (.z _relativelocation) 6.0))
    (if (>= (.z _relativelocation) 14.0)
      _)))

(event Input|ActionEvents|InputActionInteraction
  (params (Key :type Key%20Structure))
  (:Pressed
    (Utilities|FlowControl|Gate true
      (:Exit
        (bind _button_in (Timeline|Button_in PlayFromStart)
          (:Update
            (Transformation|SetRelativeTransform (Variables|Default|GetButton) (Math|Transform|Lerp(Transform) (Variables|Default|GetButton%20out) (Variables|Default|GetButton%20in) _button_in) false false)
            (Class|BPILiftDoor|BPIOpenDoor(Message) (Variables|Default|GetDoor)))
          (:Finished
            (bind _button_in_2 (Timeline|Timeline ReverseFromEnd)
              (:Update
                (Transformation|SetRelativeTransform (Variables|Default|GetButton) (Math|Transform|Lerp(Transform) (Variables|Default|GetButton%20out) (Variables|Default|GetButton%20in) _button_in_2) false false)
                (Class|BPILiftDoor|BPIOpenDoor(Message) (Variables|Default|GetDoor))))))))))

(event Input|KeyboardEvents|E
  (params (Key :type Key%20Structure))
  (:Pressed
    (Utilities|FlowControl|Gate true) ; enters at Open
  ))

(fn ConstructionScript)

(event OnComponentEndOverlap(Box)
  (params (OverlappedComponent :type Primitive%20Component%20Object%20Reference) (OtherActor :type Actor%20Object%20Reference) (OtherComp :type Primitive%20Component%20Object%20Reference) (OtherBodyIndex :type Integer))
  (Utilities|Casting|CastToALS_AnimMan_CharacterBP OtherActor)
  (Input|DisableInput (Game|GetPlayerController 0))
  (Utilities|FlowControl|Gate true) ; enters at Close
)

(event OnComponentBeginOverlap(Box)
  (params (OverlappedComponent :type Primitive%20Component%20Object%20Reference) (OtherActor :type Actor%20Object%20Reference) (OtherComp :type Primitive%20Component%20Object%20Reference) (OtherBodyIndex :type Integer) (bFromSweep :type Boolean) (SweepResult :type Hit%20Result%20Structure%20%28by%20ref%29))
  (Utilities|Casting|CastToALS_AnimMan_CharacterBP OtherActor)
  (Input|EnableInput (Game|GetPlayerController 0))
  (Utilities|FlowControl|Gate true) ; enters at Open
)

(event Input|ActionEvents|InputActionInteraction
  (params (Key :type Key%20Structure))
  (:Pressed
    (if (Variables|/Game/Blueprints/BP_Generator.BP_Generator_C|GetIsGenWrk (Variables|Default|GetAs%20BP%20Generator))
      (Utilities|FlowControl|Gate true
        (:Exit
          (bind _button_in (Timeline|Button_in Play)
            (:Update
              (Transformation|SetRelativeScale3D (Variables|Default|GetButton) (Math|Vector|MakeVector 0.0 0.0 (Math|Float|Lerp 0.6 0.45 _button_in))))
            (:Finished
              (Default|OpenDoor (Variables|Default|GetDoor))))))
      (else
        (Development|PrintString "Need to repair")))))

(fn ConstructionScript)