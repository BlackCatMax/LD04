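; BP_Button_2 is a pressable wall or panel button that opens a linked door when the generator is working.
; Box overlap opens and closes a gate, so the Interaction input only registers while something is inside the trigger.
; A press moves the Button along Y and back with two short MoveComponentTo calls, then calls OpenDoor on Door if the generator's IsGenWrk is true.
; An unconnected timeline for scaling the button is left unused.
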(event OnComponentEndOverlap(Box)
  (params (OverlappedComponent :type Primitive%20Component%20Object%20Reference) (OtherActor :type Actor%20Object%20Reference) (OtherComp :type Primitive%20Component%20Object%20Reference) (OtherBodyIndex :type Integer))
  (bind _button (Variables|Default|GetButton))
  (bind _button_2 (Variables|Default|GetButton))
  (bind _button_3 (Variables|Default|GetButton))
  (bind _button_4 (Variables|Default|GetButton))
  (bind _relativerotation (Variables|/Script/Engine.SceneComponent|GetRelativeRotation _button_4))
  (bind _relativelocation (Variables|/Script/Engine.SceneComponent|GetRelativeLocation _button_2))
  (bind _relativerotation_2 (Variables|/Script/Engine.SceneComponent|GetRelativeRotation _button_3))
  (bind _relativelocation_2 (Variables|/Script/Engine.SceneComponent|GetRelativeLocation _button))
  (Utilities|FlowControl|Gate true) ; enters at Close
)

(event OnComponentBeginOverlap(Box)
  (params (OverlappedComponent :type Primitive%20Component%20Object%20Reference) (OtherActor :type Actor%20Object%20Reference) (OtherComp :type Primitive%20Component%20Object%20Reference) (OtherBodyIndex :type Integer) (bFromSweep :type Boolean) (SweepResult :type Hit%20Result%20Structure%20%28by%20ref%29))
  (bind _button (Variables|Default|GetButton))
  (bind _button_2 (Variables|Default|GetButton))
  (bind _button_3 (Variables|Default|GetButton))
  (bind _button_4 (Variables|Default|GetButton))
  (bind _relativerotation (Variables|/Script/Engine.SceneComponent|GetRelativeRotation _button_4))
  (bind _relativelocation (Variables|/Script/Engine.SceneComponent|GetRelativeLocation _button_2))
  (bind _relativerotation_2 (Variables|/Script/Engine.SceneComponent|GetRelativeRotation _button_3))
  (bind _relativelocation_2 (Variables|/Script/Engine.SceneComponent|GetRelativeLocation _button))
  (Utilities|FlowControl|Gate true) ; enters at Open
)

(event Input|ActionEvents|InputActionInteraction
  (params (Key :type Key%20Structure :default "None"))
  (bind _button (Variables|Default|GetButton))
  (bind _button_2 (Variables|Default|GetButton))
  (bind _button_3 (Variables|Default|GetButton))
  (bind _button_4 (Variables|Default|GetButton))
  (bind _relativerotation (Variables|/Script/Engine.SceneComponent|GetRelativeRotation _button_4))
  (bind _relativelocation (Variables|/Script/Engine.SceneComponent|GetRelativeLocation _button_2))
  (bind _relativerotation_2 (Variables|/Script/Engine.SceneComponent|GetRelativeRotation _button_3))
  (bind _relativelocation_2 (Variables|/Script/Engine.SceneComponent|GetRelativeLocation _button))
  (:Pressed
    (Utilities|FlowControl|Gate true
      (:Exit
        (Components|MoveComponentTo (Variables|Default|GetButton) (Math|Vector|MakeVector (.x _relativelocation) -5.0 (.z _relativelocation)) (Math|Rotator|MakeRotator (.roll _relativerotation_2) (.pitch _relativerotation_2) (.yaw _relativerotation_2)) false false 0.2 false)
        (Components|MoveComponentTo (Variables|Default|GetButton) (Math|Vector|MakeVector (.x _relativelocation_2) 1e+01 (.z _relativelocation_2)) (Math|Rotator|MakeRotator (.roll _relativerotation) (.pitch _relativerotation) (.yaw _relativerotation)) false false 0.2 false)
        (if (Variables|/Game/Blueprints/BP_Generator.BP_Generator_C|GetIsGenWrk (Variables|Generator|GetAs%20BP%20Generator))
          (Default|OpenDoor (Variables|Door|GetDoor)))))))

(fn ConstructionScript)