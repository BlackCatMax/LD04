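; Elevator actor that raises or lowers its Elevation component once when the ALS player-type character enters its trigger box.
; The overlap only takes effect if the referenced Target's WorkButton flag is set, and a DoOnce limits it to a single one-way trip.
; MoveComponentTo eases the component over a few seconds to the relative height of an Arrow marker, keeping X and Y unchanged.
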(event OnComponentBeginOverlap(Box)
  (params (OverlappedComponent :type Primitive%20Component%20Object%20Reference) (OtherActor :type Actor%20Object%20Reference) (OtherComp :type Primitive%20Component%20Object%20Reference) (OtherBodyIndex :type Integer) (bFromSweep :type Boolean) (SweepResult :type Hit%20Result%20Structure%20%28by%20ref%29))
  (bind _elevation (Variables|Default|GetElevation))
  (bind _relativelocation (Variables|/Script/Engine.SceneComponent|GetRelativeLocation _elevation))
  (Utilities|Casting|CastToALS_AnimMan_CharacterBP OtherActor)
  (if (Variables|/Game/Maps/Maria/BP_KNOPKA.BP_KNOPKA_C|GetWork%20Button (Variables|Default|GetTarget))
    (Utilities|FlowControl|DoOnce false
      (:Completed
        (Components|MoveComponentTo (Variables|Default|GetElevation) (Math|Vector|MakeVector (.x _relativelocation) (.y _relativelocation) (.z (Variables|/Script/Engine.SceneComponent|GetRelativeLocation (Variables|Default|GetArrow)))) "0, 0, 0" true true 4.0 false)))))

(fn ConstructionScript)