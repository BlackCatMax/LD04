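; BP_NOTE1 is an interactable note that shows and removes a UI widget when E is pressed near it.
; Box overlap enables input and opens a Gate, and leaving closes the Gate, though input is enabled again rather than disabled.
; A FlipFlop behind the Gate alternates between creating the E widget while hiding the Box and removing it while showing the Box again.
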(event OnComponentBeginOverlap(Box)
  (params (OverlappedComponent :type Primitive%20Component%20Object%20Reference) (OtherActor :type Actor%20Object%20Reference) (OtherComp :type Primitive%20Component%20Object%20Reference) (OtherBodyIndex :type Integer) (bFromSweep :type Boolean) (SweepResult :type Hit%20Result%20Structure%20%28by%20ref%29))
  (bind _box (Variables|Default|GetBox))
  (Input|EnableInput (Game|GetPlayerController 0))
  (Utilities|FlowControl|Gate true) ; enters at Open
)

(event OnComponentEndOverlap(Box)
  (params (OverlappedComponent :type Primitive%20Component%20Object%20Reference) (OtherActor :type Actor%20Object%20Reference) (OtherComp :type Primitive%20Component%20Object%20Reference) (OtherBodyIndex :type Integer))
  (bind _box (Variables|Default|GetBox))
  (Input|EnableInput (Game|GetPlayerController 0))
  (Utilities|FlowControl|Gate true) ; enters at Close
)

(event Input|KeyboardEvents|E
  (params (Key :type Key%20Structure :default "None"))
  (bind _box (Variables|Default|GetBox))
  (:Pressed
    (Utilities|FlowControl|Gate true
      (:Exit
        (Utilities|FlowControl|FlipFlop
          (:A
            (bind _returnvalue (UserInterface|CreateWidget "/Game/Maps/Maria/model/E.E_C"))
            (UserInterface|Viewport|AddtoViewport _returnvalue 0)
            (Rendering|SetVisibility _box false false))
          (:B
            (Widget|RemovefromParent _returnvalue)
            (Rendering|SetVisibility _box true false)))))))

(fn ConstructionScript)