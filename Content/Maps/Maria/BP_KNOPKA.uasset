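; A pressable button actor that the ALS player character triggers with the E key when standing nearby.
; Box overlap enables and disables the actor's input for player 0, limiting the key to that area.
; Pressing E plays the ButtonIn timeline, which moves the Button component and sets the WorkButton flag on each update.
; Two MoveComponentTo nodes are left unconnected and never run.
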(event OnComponentBeginOverlap(Box)
  (params (OverlappedComponent :type Primitive%20Component%20Object%20Reference) (OtherActor :type Actor%20Object%20Reference) (OtherComp :type Primitive%20Component%20Object%20Reference) (OtherBodyIndex :type Integer) (bFromSweep :type Boolean) (SweepResult :type Hit%20Result%20Structure%20%28by%20ref%29))
  (Utilities|Casting|CastToALS_AnimMan_CharacterBP OtherActor)
  (Input|EnableInput (Game|GetPlayerController 0)))

(event OnComponentEndOverlap(Box)
  (params (OverlappedComponent :type Primitive%20Component%20Object%20Reference) (OtherActor :type Actor%20Object%20Reference) (OtherComp :type Primitive%20Component%20Object%20Reference) (OtherBodyIndex :type Integer))
  (Utilities|Casting|CastToALS_AnimMan_CharacterBP OtherActor)
  (Input|DisableInput (Game|GetPlayerController 0)))

(event Input|KeyboardEvents|E
  (params (Key :type Key%20Structure :default "None"))
  (:Pressed
    (bind _button1 (Timeline|Button%20In Play)
      (:Update
        (Transformation|SetRelativeLocation (Variables|Default|GetButton) _button1 false false)
        (Variables|Default|SetWork%20Button true)))))

(fn ConstructionScript)