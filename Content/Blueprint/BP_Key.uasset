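; BP_Key is a key pickup that the ALS_AnimMan_CharacterBP character collects by pressing E while near it.
; Overlapping Sphere1 caches the character, enables input for player 0 and opens a Gate node; leaving disables input and closes the gate.
; An E press through the open gate increments the character's HaveKeys count, prints it and destroys the key actor.
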(event OnComponentBeginOverlap(Sphere1)
  (params (OverlappedComponent :type Primitive%20Component%20Object%20Reference) (OtherActor :type Actor%20Object%20Reference) (OtherComp :type Primitive%20Component%20Object%20Reference) (OtherBodyIndex :type Integer) (bFromSweep :type Boolean) (SweepResult :type Hit%20Result%20Structure%20%28by%20ref%29))
  (bind _asals_anim_man_character_bp (Utilities|Casting|CastToALS_AnimMan_CharacterBP OtherActor))
  (Variables|Default|SetAs%20ALS%20Anim%20Man%20Character%20BP _asals_anim_man_character_bp)
  (Input|EnableInput (Game|GetPlayerController 0))
  (Utilities|FlowControl|Gate true) ; enters at Open
)

(event OnComponentEndOverlap(Sphere1)
  (params (OverlappedComponent :type Primitive%20Component%20Object%20Reference) (OtherActor :type Actor%20Object%20Reference) (OtherComp :type Primitive%20Component%20Object%20Reference) (OtherBodyIndex :type Integer))
  (bind _as_als_anim_man_character_bp (Variables|Default|GetAs%20ALS%20Anim%20Man%20Character%20BP))
  (Utilities|Casting|CastToALS_AnimMan_CharacterBP OtherActor)
  (Input|DisableInput (Game|GetPlayerController 0))
  (Utilities|FlowControl|Gate true) ; enters at Close
)

(event Input|KeyboardEvents|E
  (params (Key :type Key%20Structure :default "None"))
  (bind _as_als_anim_man_character_bp (Variables|Default|GetAs%20ALS%20Anim%20Man%20Character%20BP))
  (:Pressed
    (Utilities|FlowControl|Gate true
      (:Exit
        (bind _output_get (Variables|/Game/AdvancedLocomotionV4/Blueprints/CharacterLogic/ALS_AnimMan_CharacterBP.ALS_AnimMan_CharacterBP_C|SetHaveKeys _as_als_anim_man_character_bp (+ (Variables|/Game/AdvancedLocomotionV4/Blueprints/CharacterLogic/ALS_AnimMan_CharacterBP.ALS_AnimMan_CharacterBP_C|GetHaveKeys _as_als_anim_man_character_bp) 1)))
        (Development|PrintString (Utilities|String|ToString(Integer) _output_get))
        (Actor|DestroyActor)))))

(fn ConstructionScript)