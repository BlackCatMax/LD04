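; BP_Lock is a lock actor that takes one of the player's keys and counts toward opening a linked Gate.
; Box overlap by the ALS character toggles input and a flow gate, so E only works in range.
; Each press spends a key, reveals the Sphere and increments the Gate's LockTotal, calling OpenDoorEvent when it equals LockNeeded.
; Nothing prevents repeated use of the same lock, and debug prints remain.
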(event OnComponentBeginOverlap(Box)
  (params (OverlappedComponent :type Primitive%20Component%20Object%20Reference) (OtherActor :type Actor%20Object%20Reference) (OtherComp :type Primitive%20Component%20Object%20Reference) (OtherBodyIndex :type Integer) (bFromSweep :type Boolean) (SweepResult :type Hit%20Result%20Structure%20%28by%20ref%29))
  (bind _gate (Variables|Default|GetGate))
  (bind _asals_anim_man_character_bp (Utilities|Casting|CastToALS_AnimMan_CharacterBP OtherActor))
  (Variables|Default|SetAs%20ALS%20Anim%20Man%20Character%20BP _asals_anim_man_character_bp)
  (Input|EnableInput (Game|GetPlayerController 0))
  (Utilities|FlowControl|Gate true) ; enters at Open
)

(event OnComponentEndOverlap(Box)
  (params (OverlappedComponent :type Primitive%20Component%20Object%20Reference) (OtherActor :type Actor%20Object%20Reference) (OtherComp :type Primitive%20Component%20Object%20Reference) (OtherBodyIndex :type Integer))
  (bind _gate (Variables|Default|GetGate))
  (Utilities|Casting|CastToALS_AnimMan_CharacterBP OtherActor)
  (Input|DisableInput (Game|GetPlayerController 0))
  (Utilities|FlowControl|Gate true) ; enters at Close
)

(event Input|KeyboardEvents|E
  (params (Key :type Key%20Structure :default "None"))
  (bind _gate (Variables|Default|GetGate))
  (:Pressed
    (Utilities|FlowControl|Gate true
      (:Exit
        (if (> (Variables|/Game/AdvancedLocomotionV4/Blueprints/CharacterLogic/ALS_AnimMan_CharacterBP.ALS_AnimMan_CharacterBP_C|GetHaveKeys (Variables|Default|GetAs%20ALS%20Anim%20Man%20Character%20BP)) 0)
          (Variables|/Game/AdvancedLocomotionV4/Blueprints/CharacterLogic/ALS_AnimMan_CharacterBP.ALS_AnimMan_CharacterBP_C|SetHaveKeys (Variables|Default|GetAs%20ALS%20Anim%20Man%20Character%20BP) (- (Variables|/Game/AdvancedLocomotionV4/Blueprints/CharacterLogic/ALS_AnimMan_CharacterBP.ALS_AnimMan_CharacterBP_C|GetHaveKeys (Variables|Default|GetAs%20ALS%20Anim%20Man%20Character%20BP)) 1))
          (Development|SetHiddeninGame (Variables|Default|GetSphere) false false)
          (bind _output_get (Variables|/Game/Blueprint/BP_Gate.BP_Gate_C|SetLockTotal _gate (+ (Variables|/Game/Blueprint/BP_Gate.BP_Gate_C|GetLockTotal _gate) 1)))
          (Development|PrintString (Utilities|String|ToString(Integer) _output_get) true true "(R=1.000000,G=0.014359,B=0.000000,A=1.000000)")
          (if (== (Variables|/Game/Blueprint/BP_Gate.BP_Gate_C|GetLockNeeded _gate) _output_get)
            (Default|OpenDoorEvent _gate)
            (Development|PrintString (Utilities|String|ToString(Integer) (Variables|/Game/AdvancedLocomotionV4/Blueprints/CharacterLogic/ALS_AnimMan_CharacterBP.ALS_AnimMan_CharacterBP_C|GetHaveKeys (Variables|Default|GetAs%20ALS%20Anim%20Man%20Character%20BP))) true true "(R=0.288456,G=1.000000,B=0.000000,A=1.000000)")))))))

(fn ConstructionScript)