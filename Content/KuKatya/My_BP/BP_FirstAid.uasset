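; First aid pickup that an ALS_AnimMan character collects by pressing E near it.
; Box overlap stores the character, enables player 0 input on the actor, shows TextE and opens a gate; end overlap disables input and closes the gate.
; E sets the character's HaveLoot flag, then destroys the pickup through the gate.
; End overlap also sets TextE visible, so the prompt is never hidden here.
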(event OnComponentEndOverlap(Box)
  (params (OverlappedComponent :type Primitive%20Component%20Object%20Reference) (OtherActor :type Actor%20Object%20Reference) (OtherComp :type Primitive%20Component%20Object%20Reference) (OtherBodyIndex :type Integer))
  (Utilities|Casting|CastToALS_AnimMan_CharacterBP OtherActor)
  (Input|DisableInput (Game|GetPlayerController 0))
  (Rendering|SetVisibility (Variables|Default|GetText_E) true false)
  (Utilities|FlowControl|Gate true) ; enters at Close
)

(event OnComponentBeginOverlap(Box)
  (params (OverlappedComponent :type Primitive%20Component%20Object%20Reference) (OtherActor :type Actor%20Object%20Reference) (OtherComp :type Primitive%20Component%20Object%20Reference) (OtherBodyIndex :type Integer) (bFromSweep :type Boolean) (SweepResult :type Hit%20Result%20Structure%20%28by%20ref%29))
  (bind _asals_anim_man_character_bp (Utilities|Casting|CastToALS_AnimMan_CharacterBP OtherActor))
  (Variables|Default|SetAlsAnimMen _asals_anim_man_character_bp)
  (Input|EnableInput (Game|GetPlayerController 0))
  (Rendering|SetVisibility (Variables|Default|GetText_E) true false)
  (Utilities|FlowControl|Gate true) ; enters at Open
)

(event Input|KeyboardEvents|E
  (params (Key :type Key%20Structure :default "None"))
  (:Pressed
    (Variables|/Game/AdvancedLocomotionV4/Blueprints/CharacterLogic/ALS_AnimMan_CharacterBP.ALS_AnimMan_CharacterBP_C|SetHaveLoot (Variables|Default|GetAlsAnimMen) true)
    (Utilities|FlowControl|Gate true
      (:Exit
        (Actor|DestroyActor)))))

(fn ConstructionScript)