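; BP_Note2Fl2 is an interactable note actor that lets the player open and close a note widget with the E key.
; Overlap of its Box by an ALS_AnimMan character enables input and opens a Gate, while leaving disables input and closes it.
; A FlipFlop alternates between creating a new WidgetNote2Kukatya on screen and hiding it without removal.
; Both overlap events set the TextRender invisible.
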(event OnComponentBeginOverlap(Box)
  (params (OverlappedComponent :type Primitive%20Component%20Object%20Reference) (OtherActor :type Actor%20Object%20Reference) (OtherComp :type Primitive%20Component%20Object%20Reference) (OtherBodyIndex :type Integer) (bFromSweep :type Boolean) (SweepResult :type Hit%20Result%20Structure%20%28by%20ref%29))
  (bind _asals_anim_man_character_bp (Utilities|Casting|CastToALS_AnimMan_CharacterBP OtherActor))
  (Variables|Default|SetAs%20ALS%20Anim%20Man%20Character%20BP _asals_anim_man_character_bp)
  (Input|EnableInput (Game|GetPlayerController 0))
  (Rendering|SetVisibility (Variables|Default|GetTextRender) false false)
  (Utilities|FlowControl|Gate true) ; enters at Open
)

(event OnComponentEndOverlap(Box)
  (params (OverlappedComponent :type Primitive%20Component%20Object%20Reference) (OtherActor :type Actor%20Object%20Reference) (OtherComp :type Primitive%20Component%20Object%20Reference) (OtherBodyIndex :type Integer))
  (Utilities|Casting|CastToALS_AnimMan_CharacterBP OtherActor)
  (Input|DisableInput (Game|GetPlayerController 0))
  (Rendering|SetVisibility (Variables|Default|GetTextRender) false false)
  (Utilities|FlowControl|Gate true) ; enters at Close
)

(event Input|KeyboardEvents|E
  (params (Key :type Key%20Structure :default "None"))
  (:Pressed
    (Utilities|FlowControl|Gate true
      (:Exit
        (Utilities|FlowControl|FlipFlop
          (:A
            (bind _returnvalue (UserInterface|CreateWidget "/Game/KuKatya/My_Widget/WidgetNote2Kukatya.WidgetNote2Kukatya_C"))
            (UserInterface|Viewport|AddtoViewport _returnvalue 0))
          (:B
            (Widget|SetVisibility _returnvalue "Hidden")))))))

(fn ConstructionScript)