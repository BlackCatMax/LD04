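; Loot pickup actor that the ALS character collects by pressing E while inside its Box trigger.
; Overlap stores the character, enables input, shows the TextE prompt and opens a gate; leaving reverses the input, prompt and gate.
; E sets HaveLoot, then through the open gate increments the character's AmountOfLoot and destroys the actor.
; A nonzero count then adds a newly created WBP_Loot widget to the viewport on each pickup.
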(event OnComponentEndOverlap(Box)
  (params (OverlappedComponent :type Primitive%20Component%20Object%20Reference) (OtherActor :type Actor%20Object%20Reference) (OtherComp :type Primitive%20Component%20Object%20Reference) (OtherBodyIndex :type Integer))
  (bind _alsanimmen (Variables|Default|GetAlsAnimMen))
  (Utilities|Casting|CastToALS_AnimMan_CharacterBP OtherActor)
  (Input|DisableInput (Game|GetPlayerController 0))
  (Rendering|SetVisibility (Variables|Default|GetText_E) false false)
  (Utilities|FlowControl|Gate true) ; enters at Close
)

(event OnComponentBeginOverlap(Box)
  (params (OverlappedComponent :type Primitive%20Component%20Object%20Reference) (OtherActor :type Actor%20Object%20Reference) (OtherComp :type Primitive%20Component%20Object%20Reference) (OtherBodyIndex :type Integer) (bFromSweep :type Boolean) (SweepResult :type Hit%20Result%20Structure%20%28by%20ref%29))
  (bind _asals_anim_man_character_bp (Utilities|Casting|CastToALS_AnimMan_CharacterBP OtherActor))
  (Variables|Default|SetAlsAnimMen _asals_anim_man_character_bp)
  (Input|EnableInput (Game|GetPlayerController 0))
  (Rendering|SetVisibility (Variables|Default|GetText_E) true false)
  (Utilities|FlowControl|Gate true) ; enters at Open
)

(event Input|KeyboardEvents|E
  (params (Key :type Key%20Structure :default "None"))
  (bind _alsanimmen (Variables|Default|GetAlsAnimMen))
  (:Pressed
    (Variables|/Game/AdvancedLocomotionV4/Blueprints/CharacterLogic/ALS_AnimMan_CharacterBP.ALS_AnimMan_CharacterBP_C|SetHaveLoot (Variables|Default|GetAlsAnimMen) true)
    (Utilities|FlowControl|Gate true
      (:Exit
        (Variables|/Game/AdvancedLocomotionV4/Blueprints/CharacterLogic/ALS_AnimMan_CharacterBP.ALS_AnimMan_CharacterBP_C|SetAmountOfLoot _alsanimmen (+ (Variables|/Game/AdvancedLocomotionV4/Blueprints/CharacterLogic/ALS_AnimMan_CharacterBP.ALS_AnimMan_CharacterBP_C|GetAmountOfLoot _alsanimmen) 1))
        (Actor|DestroyActor)
        (if (Math|Conversions|ToBoolean(Integer) (Variables|/Game/AdvancedLocomotionV4/Blueprints/CharacterLogic/ALS_AnimMan_CharacterBP.ALS_AnimMan_CharacterBP_C|GetAmountOfLoot _alsanimmen))
          (bind _returnvalue (UserInterface|CreateWidget "/Game/KuKatya/My_Widget/WBP_Loot.WBP_Loot_C"))
          (UserInterface|Viewport|AddtoViewport _returnvalue 0))))))

(fn ConstructionScript)