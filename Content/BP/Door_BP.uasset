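; Interactive door actor that the player opens and closes with the E key while inside its trigger box.
; The Box overlap shows a text prompt and enables input for player 0, undoing both on exit.
; E plays or reverses a timeline that drives door yaw from negated Alpha.
; DoorTime blocks presses until the timeline finishes, and DoorOpen, true at zero Alpha, picks the direction.
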(event OnComponentBeginOverlap(Box)
  (params (OverlappedComponent :type Primitive%20Component%20Object%20Reference) (OtherActor :type Actor%20Object%20Reference) (OtherComp :type Primitive%20Component%20Object%20Reference) (OtherBodyIndex :type Integer) (bFromSweep :type Boolean) (SweepResult :type Hit%20Result%20Structure%20%28by%20ref%29))
  (Input|EnableInput (Game|GetPlayerController 0))
  (Rendering|SetVisibility (Variables|Default|GetTextRender) true false))

(event OnComponentEndOverlap(Box)
  (params (OverlappedComponent :type Primitive%20Component%20Object%20Reference) (OtherActor :type Actor%20Object%20Reference) (OtherComp :type Primitive%20Component%20Object%20Reference) (OtherBodyIndex :type Integer))
  (Input|DisableInput (Game|GetPlayerController 0))
  (Rendering|SetVisibility (Variables|Default|GetTextRender) false false))

(event EventBeginPlay)

(event Collision|EventActorBeginOverlap
  (params (OtherActor :type Actor%20Object%20Reference)))

(event EventTick
  (params (DeltaSeconds :type Float%20%28single-precision%29)))

(event Input|KeyboardEvents|E
  (params (Key :type Key%20Structure :default "None"))
  (:Pressed
    (if (Variables|Default|GetDoor_Time)
      (if (Variables|Default|GetDoor_Open)
        (Variables|Default|SetDoor_Time false)
        (bind _alpha (Timeline|Timeline_Door Play)
          (:Update
            (Transformation|SetRelativeRotation (Variables|Default|GetDoor) (Math|Rotator|MakeRotator 0.0 0.0 (* _alpha -1.0)) false false)
            (Variables|Default|SetDoor_Open (not (> _alpha 0.0))))
          (:Finished
            (Variables|Default|SetDoor_Time true)))
        (else
          (Variables|Default|SetDoor_Time false)
          (Timeline|Timeline_Door ReverseFromEnd))))))

(fn ConstructionScript)