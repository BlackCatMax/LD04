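; Configurable door actor that the 1 key toggles between playing and reversing its motion.
; The DoorMoving timeline drives the Center component by DoorType: uniform scaling, sliding along X, or yaw swinging.
; Swing direction flips according to the dot product of door and player forward vectors, re-evaluated on every timeline update.
; The construction script sets the door mesh and offset, and applies color and metallic values to door and frame through dynamic materials.
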(event Collision|EventActorBeginOverlap
  (params (OtherActor :type Actor%20Object%20Reference)))

(event EventTick
  (params (DeltaSeconds :type Float%20%28single-precision%29)))

(event EventBeginPlay)

(event Input|KeyboardEvents|1
  (params (Key :type Key%20Structure :default "None"))
  (bind _center (Variables|Default|GetCenter))
  (:Pressed
    (Utilities|FlowControl|FlipFlop
      (:A
        (Components|Timeline|SetPlayRate (Variables|Default|GetDoorMoving) (Variables|DoorMoving|GetNew%20Rate))
        (bind _alpha (Timeline|DoorMoving Play)
          (:Update
            (switch int (Variables|DoorCustomization|GetDoorType)
              (:0
                (Transformation|SetRelativeScale3D _center (Math|Vector|MakeVector (Math|Float|Lerp 0.1 0.2 _alpha) (Math|Float|Lerp 0.1 0.2 _alpha) (Math|Float|Lerp 0.1 0.2 _alpha))))
              (:1
                (Transformation|SetRelativeLocation _center (Math|Vector|MakeVector (Math|Float|Lerp (Variables|DoorMoving|GetStart%20Location) (Variables|DoorMoving|GetEnd%20Location) _alpha) 15.0 0.0) false false))
              (:2
                (if (> (Math|Vector|DotProduct (Transformation|GetActorForwardVector) (Transformation|GetActorForwardVector (Game|GetPlayerCharacter 0))) 0.0)
                  (Transformation|SetRelativeRotation _center (Math|Rotator|MakeRotator 0.0 0.0 (Math|Float|Lerp (Variables|DoorMoving|GetStart%20Door%20Position) (Variables|DoorMoving|GetEnd%20Door%20Position) _alpha)) false false)
                  (else
                    (Transformation|SetRelativeRotation _center (Math|Rotator|MakeRotator 0.0 0.0 (* (Math|Float|Lerp (Variables|DoorMoving|GetStart%20Door%20Position) (Variables|DoorMoving|GetEnd%20Door%20Position) _alpha) -1.0)) false false))))))))
      (:B
        (Timeline|DoorMoving Reverse)))))

(fn ConstructionScript
  (Utilities|FlowControl|Sequence
    (:then_0
      (bind _returnvalue (Rendering|Material|CreateDynamicMaterialInstance (Variables|Default|GetDoor) 0 (Variables|DoorCustomization|GetSource%20MaterialDoor) "None" :!class /Script/Engine.PrimitiveComponent))
      (Rendering|Material|SetVectorParameterValue _returnvalue "Color" (Variables|DoorCustomization|GetDoorColor) :!class /Script/Engine.MaterialInstanceDynamic)
      (Rendering|Material|SetScalarParameterValue _returnvalue "Metallic" (Variables|DoorCustomization|GetDoor%20Metallic) :!class /Script/Engine.MaterialInstanceDynamic))
    (:then_1
      (bind _returnvalue_2 (Rendering|Material|CreateDynamicMaterialInstance (Variables|Default|GetFrame) 0 (Variables|DoorCustomization|GetSource%20MaterialFrame) "None" :!class /Script/Engine.PrimitiveComponent))
      (Rendering|Material|SetVectorParameterValue _returnvalue_2 "Color" (Variables|DoorCustomization|GetFrame%20Color) :!class /Script/Engine.MaterialInstanceDynamic)
      (Rendering|Material|SetScalarParameterValue _returnvalue_2 "Metallic" (Variables|DoorCustomization|GetFrame%20Metallic) :!class /Script/Engine.MaterialInstanceDynamic))
    (:then_2
      (Components|StaticMesh|SetStaticMesh (Variables|Default|GetDoor) (Variables|DoorCustomization|GetDoor%20Mesh))
      (Transformation|SetRelativeLocation (Variables|Default|GetDoor) (Variables|DoorCustomization|GetDoor%20New%20Location) false false))
    (:then_3
      (Variables|DoorCustomization|SetDoorType (Variables|DoorCustomization|GetDoorType)))))